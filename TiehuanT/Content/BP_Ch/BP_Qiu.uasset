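; BP_Qiu is a ball actor that duplicates itself when its 分裂 (split) event is called.
; After a short delay, if off cooldown, it spawns a copy at its transform with the same velocity.
; Both balls play a timeline that grows their scale from half to full, and its completion clears the split cooldown.
; The sphere overlap handler loops over the other actor's tags but does nothing with them.
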(event OnComponentBeginOverlap(Sphere)
  (params (OverlappedComponent :type Primitive%20Component%20Object%20Reference) (OtherActor :type Actor%20Object%20Reference) (OtherComp :type Primitive%20Component%20Object%20Reference) (OtherBodyIndex :type Integer) (bFromSweep :type Boolean) (SweepResult :type Hit%20Result%20Structure%20%28by%20ref%29))
  (for _array_element (Variables|/Script/Engine.Actor|GetTags OtherActor)
    _))

(event Custom|分裂
  (Utilities|FlowControl|Delay 0.2)
  (if (not (Variables|Default|Get分裂冷却))
    (bind _returnvalue (Game|SpawnActorfromClass "BP_Qiu_C" (Transformation|GetActorTransform) "Undefined" "MultiplyWithRoot" 0 0))
    (Utilities|FlowControl|Sequence
      (:then_0
        (Variables|BP_Qiu_C|Set分裂冷却 _returnvalue true)
        (Physics|SetPhysicsLinearVelocity (Variables|BP_Qiu_C|GetSphere1 _returnvalue) (Transformation|GetVelocity) false "None")
        (CallFunction|动画 _returnvalue))
      (:then_1
        (Variables|Default|Set分裂冷却 true)
        (bind _新建轨道_0 (Timeline|时间轴 PlayFromStart)
          (:Update
            (Transformation|SetActorScale3D (Math|Conversions|ToVector(Float) (Math|Float|Lerp 0.5 1.0 _新建轨道_0))))
          (:Finished
            (Variables|Default|Set分裂冷却 false)))))))

(event Custom|动画
  (bind _新建轨道_0 (Timeline|时间轴 PlayFromStart)
    (:Update
      (Transformation|SetActorScale3D (Math|Conversions|ToVector(Float) (Math|Float|Lerp 0.5 1.0 _新建轨道_0))))
    (:Finished
      (Variables|Default|Set分裂冷却 false))))

(event EventBeginPlay)

(event Collision|EventActorBeginOverlap
  (params (OtherActor :type Actor%20Object%20Reference)))

(event EventTick
  (params (DeltaSeconds :type Float%20%28single-precision%29)))

(fn ConstructionScript)