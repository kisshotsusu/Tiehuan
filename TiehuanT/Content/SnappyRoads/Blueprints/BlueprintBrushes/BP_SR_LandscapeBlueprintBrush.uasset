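; Landscape Blueprint brush that shapes terrain and paints a weightmap layer around selected BP_SnappyRoad actors.
; Initialization sizes an orthographic scene capture to the landscape, creates render targets and fills MPC_SR_Landscape.
; The heightmap pass captures road depth at forced LOD 0, jump-floods it into a blurred, cached distance field, then blends it through M_SR_SimpleBrush.
; The weightmap pass reuses that depth and cache to paint with falloff.
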(event Custom|SaveRT
  (Rendering|ExportRenderTarget (Variables|Debug|RTs|GetDepth_RT) "c:\\tmp\\" "1.png"))

(event Custom|UpdateLandscape
  (Landscape|RequestLandscapeUpdate))

(event Custom|UpdateTransform
  (Variables|Debug|SetWorldSize (Math|Vector|MakeVector (* (.X (Utilities|Struct|BreakIntPoint (stale EventInitialize _output_get_2))) (.X (Math|Vector|BreakVector (.Scale (Math|Transform|BreakTransform (stale EventInitialize _output_get)))))) (* (.Y (Utilities|Struct|BreakIntPoint (stale EventInitialize _output_get_2))) (.Y (Math|Vector|BreakVector (.Scale (Math|Transform|BreakTransform (stale EventInitialize _output_get)))))) 0.512))
  (Variables|/Script/Engine.SceneCaptureComponent2D|SetOrthoWidth (Variables|Default|GetSceneCaptureComponent2D) (Math|Float|Max(Float) (* (.X (Utilities|Struct|BreakIntPoint (stale EventInitialize _output_get_3))) (.X (Math|Vector|BreakVector (.Scale (Math|Transform|BreakTransform (stale EventInitialize _output_get)))))) (* (.Y (Utilities|Struct|BreakIntPoint (stale EventInitialize _output_get_3))) (.Y (Math|Vector|BreakVector (.Scale (Math|Transform|BreakTransform (stale EventInitialize _output_get))))))))
  (Variables|Debug|SetLSZLocation (.Z (Math|Vector|BreakVector (.Location (Math|Transform|BreakTransform (stale EventInitialize _output_get))))))
  (Variables|Debug|SetLSZScale (/ (.Z (Math|Vector|BreakVector (.Scale (Math|Transform|BreakTransform (stale EventInitialize _output_get))))) 128.0))
  (Utilities|InitZOffset)
  (Transformation|SetWorldLocation (Variables|Default|GetSceneCaptureComponent2D) (Math|Vector|MakeVector (.X (Math|Vector|BreakVector (+ (.Location (Math|Transform|BreakTransform (stale EventInitialize _output_get))) (Math|Transform|TransformLocation (Math|Transform|MakeTransform "0, 0, 0" (.Rotation (Math|Transform|BreakTransform (stale EventInitialize _output_get)))) (* (- (Math|Vector|MakeVector (* (.X (Utilities|Struct|BreakIntPoint (stale EventInitialize _output_get_3))) (.X (Math|Vector|BreakVector (.Scale (Math|Transform|BreakTransform (stale EventInitialize _output_get)))))) (* (.Y (Utilities|Struct|BreakIntPoint (stale EventInitialize _output_get_3))) (.Y (Math|Vector|BreakVector (.Scale (Math|Transform|BreakTransform (stale EventInitialize _output_get)))))) 0.512) (.Scale (Math|Transform|BreakTransform (stale EventInitialize _output_get)))) 0.5))))) (.Y (Math|Vector|BreakVector (+ (.Location (Math|Transform|BreakTransform (stale EventInitialize _output_get))) (Math|Transform|TransformLocation (Math|Transform|MakeTransform "0, 0, 0" (.Rotation (Math|Transform|BreakTransform (stale EventInitialize _output_get)))) (* (- (Math|Vector|MakeVector (* (.X (Utilities|Struct|BreakIntPoint (stale EventInitialize _output_get_3))) (.X (Math|Vector|BreakVector (.Scale (Math|Transform|BreakTransform (stale EventInitialize _output_get)))))) (* (.Y (Utilities|Struct|BreakIntPoint (stale EventInitialize _output_get_3))) (.Y (Math|Vector|BreakVector (.Scale (Math|Transform|BreakTransform (stale EventInitialize _output_get)))))) 0.512) (.Scale (Math|Transform|BreakTransform (stale EventInitialize _output_get)))) 0.5))))) 5e+04) false false)
  (Transformation|SetActorRotation (Math|Rotator|MakeRotator 0.0 0.0 (.Yaw (Math|Rotator|BreakRotator (.Rotation (Math|Transform|BreakTransform (stale EventInitialize _output_get)))))))
  (Utilities|InitRTs))

(event Custom|SelectAllRoads
  (bind _scenecapturecomponent2d (Variables|Default|GetSceneCaptureComponent2D))
  ;[1 1 1] SelectAllRoads
  (Rendering|SceneCapture|ClearShowOnlyComponents _scenecapturecomponent2d)
  (Class|SceneCaptureComponent|ClearHiddenComponents _scenecapturecomponent2d)
  (bind _outactors (Actor|GetAllActorsOfClass "/Game/SnappyRoads/Blueprints/BP_SnappyRoad.BP_SnappyRoad_C"))
  (for _array_element _outactors
    (Rendering|SceneCapture|ShowOnlyActorComponents _scenecapturecomponent2d _array_element false)
    (Utilities|Array|AddUnique (Variables|Selection|GetSelectedRoads) (Utilities|ResolveSoftReference _array_element))
    (Variables|Default|SetUpdateNeeded! true)
    (Variables|Selection|SetSalectAllRoads! false))
  (Development|PrintString "Done!"))

(event Custom|Test
  ;[1 1 1] Test
  (Game|SpawnActorfromClass "BP_SR_LandscapeBlueprintBrush_C" (Math|Transform|MakeTransform (+ (Transformation|GetActorLocation) "0, 0,100.000000") "0, 0, 0" "1.000000,1.000000,1.000000") "Undefined" 0 0))

(event Custom|ReInit
  (Utilities|FlowControl|Sequence
    (:then_0
      (Rendering|Material|SetScalarParameterValue "/Game/SnappyRoads/Blueprints/BlueprintBrushes/MPC_SR_Landscape.MPC_SR_Landscape" "RTResX" (Math|Conversions|ToFloat(Integer) (.X (Utilities|Struct|BreakIntPoint (stale EventInitialize _output_get_3)))) :!class /Script/Engine.KismetMaterialLibrary)
      (Rendering|Material|SetScalarParameterValue "/Game/SnappyRoads/Blueprints/BlueprintBrushes/MPC_SR_Landscape.MPC_SR_Landscape" "RTResY" (Math|Conversions|ToFloat(Integer) (.Y (Utilities|Struct|BreakIntPoint (stale EventInitialize _output_get_3)))) :!class /Script/Engine.KismetMaterialLibrary)
      (Rendering|Material|SetScalarParameterValue "/Game/SnappyRoads/Blueprints/BlueprintBrushes/MPC_SR_Landscape.MPC_SR_Landscape" "LSQuadsX" (Math|Conversions|ToFloat(Integer) (.X (Utilities|Struct|BreakIntPoint (stale EventInitialize _output_get_2)))) :!class /Script/Engine.KismetMaterialLibrary)
      (Rendering|Material|SetScalarParameterValue "/Game/SnappyRoads/Blueprints/BlueprintBrushes/MPC_SR_Landscape.MPC_SR_Landscape" "LSQuadsY" (Math|Conversions|ToFloat(Integer) (.Y (Utilities|Struct|BreakIntPoint (stale EventInitialize _output_get_2)))) :!class /Script/Engine.KismetMaterialLibrary)
      (Rendering|Material|SetScalarParameterValue "/Game/SnappyRoads/Blueprints/BlueprintBrushes/MPC_SR_Landscape.MPC_SR_Landscape" "WorldSizeX" (* (.X (Utilities|Struct|BreakIntPoint (stale EventInitialize _output_get_2))) (.x (.Scale (Math|Transform|BreakTransform (stale EventInitialize _output_get))))) :!class /Script/Engine.KismetMaterialLibrary)
      (Rendering|Material|SetScalarParameterValue "/Game/SnappyRoads/Blueprints/BlueprintBrushes/MPC_SR_Landscape.MPC_SR_Landscape" "WorldSizeY" (* (.Y (Utilities|Struct|BreakIntPoint (stale EventInitialize _output_get_2))) (.y (.Scale (Math|Transform|BreakTransform (stale EventInitialize _output_get))))) :!class /Script/Engine.KismetMaterialLibrary)
      (Rendering|Material|SetScalarParameterValue "/Game/SnappyRoads/Blueprints/BlueprintBrushes/MPC_SR_Landscape.MPC_SR_Landscape" "LandscapeZScale" (.z (.Location (Math|Transform|BreakTransform (stale EventInitialize _output_get)))) :!class /Script/Engine.KismetMaterialLibrary)
      (Rendering|Material|SetScalarParameterValue "/Game/SnappyRoads/Blueprints/BlueprintBrushes/MPC_SR_Landscape.MPC_SR_Landscape" "LandscapeZLocation" (/ (.z (.Scale (Math|Transform|BreakTransform (stale EventInitialize _output_get)))) 128.0) :!class /Script/Engine.KismetMaterialLibrary)
      (Development|PrintString (Utilities|String|Append (Utilities|String|ToString(Float) (* (.X (Utilities|Struct|BreakIntPoint (stale EventInitialize _output_get_2))) (.x (.Scale (Math|Transform|BreakTransform (stale EventInitialize _output_get)))))) "::" (Utilities|String|ToString(Float) (* (.Y (Utilities|Struct|BreakIntPoint (stale EventInitialize _output_get_2))) (.y (.Scale (Math|Transform|BreakTransform (stale EventInitialize _output_get)))))))))
    (:then_1
      (Variables|Debug|SetWorldSize (Math|Vector|MakeVector (* (.X (Utilities|Struct|BreakIntPoint (stale EventInitialize _output_get_2))) (.X (Math|Vector|BreakVector (.Scale (Math|Transform|BreakTransform (stale EventInitialize _output_get)))))) (* (.Y (Utilities|Struct|BreakIntPoint (stale EventInitialize _output_get_2))) (.Y (Math|Vector|BreakVector (.Scale (Math|Transform|BreakTransform (stale EventInitialize _output_get)))))) 0.512))
      (Variables|/Script/Engine.SceneCaptureComponent2D|SetOrthoWidth (Variables|Default|GetSceneCaptureComponent2D) (Math|Float|Max(Float) (* (.X (Utilities|Struct|BreakIntPoint (stale EventInitialize _output_get_3))) (.X (Math|Vector|BreakVector (.Scale (Math|Transform|BreakTransform (stale EventInitialize _output_get)))))) (* (.Y (Utilities|Struct|BreakIntPoint (stale EventInitialize _output_get_3))) (.Y (Math|Vector|BreakVector (.Scale (Math|Transform|BreakTransform (stale EventInitialize _output_get))))))))
      (Variables|Debug|SetLSZLocation (.Z (Math|Vector|BreakVector (.Location (Math|Transform|BreakTransform (stale EventInitialize _output_get))))))
      (Variables|Debug|SetLSZScale (/ (.Z (Math|Vector|BreakVector (.Scale (Math|Transform|BreakTransform (stale EventInitialize _output_get))))) 128.0))
      (Utilities|InitZOffset)
      (Transformation|SetWorldLocation (Variables|Default|GetSceneCaptureComponent2D) (Math|Vector|MakeVector (.X (Math|Vector|BreakVector (+ (.Location (Math|Transform|BreakTransform (stale EventInitialize _output_get))) (Math|Transform|TransformLocation (Math|Transform|MakeTransform "0, 0, 0" (.Rotation (Math|Transform|BreakTransform (stale EventInitialize _output_get)))) (* (- (Math|Vector|MakeVector (* (.X (Utilities|Struct|BreakIntPoint (stale EventInitialize _output_get_3))) (.X (Math|Vector|BreakVector (.Scale (Math|Transform|BreakTransform (stale EventInitialize _output_get)))))) (* (.Y (Utilities|Struct|BreakIntPoint (stale EventInitialize _output_get_3))) (.Y (Math|Vector|BreakVector (.Scale (Math|Transform|BreakTransform (stale EventInitialize _output_get)))))) 0.512) (.Scale (Math|Transform|BreakTransform (stale EventInitialize _output_get)))) 0.5))))) (.Y (Math|Vector|BreakVector (+ (.Location (Math|Transform|BreakTransform (stale EventInitialize _output_get))) (Math|Transform|TransformLocation (Math|Transform|MakeTransform "0, 0, 0" (.Rotation (Math|Transform|BreakTransform (stale EventInitialize _output_get)))) (* (- (Math|Vector|MakeVector (* (.X (Utilities|Struct|BreakIntPoint (stale EventInitialize _output_get_3))) (.X (Math|Vector|BreakVector (.Scale (Math|Transform|BreakTransform (stale EventInitialize _output_get)))))) (* (.Y (Utilities|Struct|BreakIntPoint (stale EventInitialize _output_get_3))) (.Y (Math|Vector|BreakVector (.Scale (Math|Transform|BreakTransform (stale EventInitialize _output_get)))))) 0.512) (.Scale (Math|Transform|BreakTransform (stale EventInitialize _output_get)))) 0.5))))) 5e+04) false false)
      (Transformation|SetActorRotation (Math|Rotator|MakeRotator 0.0 0.0 (.Yaw (Math|Rotator|BreakRotator (.Rotation (Math|Transform|BreakTransform (stale EventInitialize _output_get)))))))
      (Utilities|InitRTs))))

(event EventBeginPlay
  (|CallParentFunction))

(event Collision|EventActorBeginOverlap
  (params (OtherActor :type Actor%20Object%20Reference))
  (|CallParentFunction OtherActor))

(event EventTick
  (params (DeltaSeconds :type Float%20%28single-precision%29))
  (|CallParentFunction DeltaSeconds))

(event EventInitialize
  (params (InLandscapeTransform :type Transform%20%28by%20ref%29) (InLandscapeSize :type Int%20Point%20Structure%20%28by%20ref%29) (InLandscapeRenderTargetSize :type Int%20Point%20Structure%20%28by%20ref%29))
  (bind _output_get (Variables|Debug|SetLSTransform InLandscapeTransform))
  (bind _output_get_2 (Variables|Debug|SetLSSize InLandscapeSize))
  (bind _output_get_3 (Variables|Debug|SetLSRTSize InLandscapeRenderTargetSize))
  (Utilities|FlowControl|Sequence
    (:then_0
      (Rendering|Material|SetScalarParameterValue "/Game/SnappyRoads/Blueprints/BlueprintBrushes/MPC_SR_Landscape.MPC_SR_Landscape" "RTResX" (Math|Conversions|ToFloat(Integer) (.X (Utilities|Struct|BreakIntPoint _output_get_3))) :!class /Script/Engine.KismetMaterialLibrary)
      (Rendering|Material|SetScalarParameterValue "/Game/SnappyRoads/Blueprints/BlueprintBrushes/MPC_SR_Landscape.MPC_SR_Landscape" "RTResY" (Math|Conversions|ToFloat(Integer) (.Y (Utilities|Struct|BreakIntPoint _output_get_3))) :!class /Script/Engine.KismetMaterialLibrary)
      (Rendering|Material|SetScalarParameterValue "/Game/SnappyRoads/Blueprints/BlueprintBrushes/MPC_SR_Landscape.MPC_SR_Landscape" "LSQuadsX" (Math|Conversions|ToFloat(Integer) (.X (Utilities|Struct|BreakIntPoint _output_get_2))) :!class /Script/Engine.KismetMaterialLibrary)
      (Rendering|Material|SetScalarParameterValue "/Game/SnappyRoads/Blueprints/BlueprintBrushes/MPC_SR_Landscape.MPC_SR_Landscape" "LSQuadsY" (Math|Conversions|ToFloat(Integer) (.Y (Utilities|Struct|BreakIntPoint _output_get_2))) :!class /Script/Engine.KismetMaterialLibrary)
      (Rendering|Material|SetScalarParameterValue "/Game/SnappyRoads/Blueprints/BlueprintBrushes/MPC_SR_Landscape.MPC_SR_Landscape" "WorldSizeX" (* (.X (Utilities|Struct|BreakIntPoint _output_get_2)) (.x (.Scale (Math|Transform|BreakTransform _output_get)))) :!class /Script/Engine.KismetMaterialLibrary)
      (Rendering|Material|SetScalarParameterValue "/Game/SnappyRoads/Blueprints/BlueprintBrushes/MPC_SR_Landscape.MPC_SR_Landscape" "WorldSizeY" (* (.Y (Utilities|Struct|BreakIntPoint _output_get_2)) (.y (.Scale (Math|Transform|BreakTransform _output_get)))) :!class /Script/Engine.KismetMaterialLibrary)
      (Rendering|Material|SetScalarParameterValue "/Game/SnappyRoads/Blueprints/BlueprintBrushes/MPC_SR_Landscape.MPC_SR_Landscape" "LandscapeZScale" (.z (.Location (Math|Transform|BreakTransform _output_get))) :!class /Script/Engine.KismetMaterialLibrary)
      (Rendering|Material|SetScalarParameterValue "/Game/SnappyRoads/Blueprints/BlueprintBrushes/MPC_SR_Landscape.MPC_SR_Landscape" "LandscapeZLocation" (/ (.z (.Scale (Math|Transform|BreakTransform _output_get))) 128.0) :!class /Script/Engine.KismetMaterialLibrary)
      (Development|PrintString (Utilities|String|Append (Utilities|String|ToString(Float) (* (.X (Utilities|Struct|BreakIntPoint _output_get_2)) (.x (.Scale (Math|Transform|BreakTransform _output_get))))) "::" (Utilities|String|ToString(Float) (* (.Y (Utilities|Struct|BreakIntPoint _output_get_2)) (.y (.Scale (Math|Transform|BreakTransform _output_get))))))))
    (:then_1
      (Variables|Debug|SetWorldSize (Math|Vector|MakeVector (* (.X (Utilities|Struct|BreakIntPoint _output_get_2)) (.X (Math|Vector|BreakVector (.Scale (Math|Transform|BreakTransform _output_get))))) (* (.Y (Utilities|Struct|BreakIntPoint _output_get_2)) (.Y (Math|Vector|BreakVector (.Scale (Math|Transform|BreakTransform _output_get))))) 0.512))
      (Variables|/Script/Engine.SceneCaptureComponent2D|SetOrthoWidth (Variables|Default|GetSceneCaptureComponent2D) (Math|Float|Max(Float) (* (.X (Utilities|Struct|BreakIntPoint _output_get_3)) (.X (Math|Vector|BreakVector (.Scale (Math|Transform|BreakTransform _output_get))))) (* (.Y (Utilities|Struct|BreakIntPoint _output_get_3)) (.Y (Math|Vector|BreakVector (.Scale (Math|Transform|BreakTransform _output_get)))))))
      (Variables|Debug|SetLSZLocation (.Z (Math|Vector|BreakVector (.Location (Math|Transform|BreakTransform _output_get)))))
      (Variables|Debug|SetLSZScale (/ (.Z (Math|Vector|BreakVector (.Scale (Math|Transform|BreakTransform _output_get)))) 128.0))
      (Utilities|InitZOffset)
      (Transformation|SetWorldLocation (Variables|Default|GetSceneCaptureComponent2D) (Math|Vector|MakeVector (.X (Math|Vector|BreakVector (+ (.Location (Math|Transform|BreakTransform _output_get)) (Math|Transform|TransformLocation (Math|Transform|MakeTransform "0, 0, 0" (.Rotation (Math|Transform|BreakTransform _output_get))) (* (- (Math|Vector|MakeVector (* (.X (Utilities|Struct|BreakIntPoint _output_get_3)) (.X (Math|Vector|BreakVector (.Scale (Math|Transform|BreakTransform _output_get))))) (* (.Y (Utilities|Struct|BreakIntPoint _output_get_3)) (.Y (Math|Vector|BreakVector (.Scale (Math|Transform|BreakTransform _output_get))))) 0.512) (.Scale (Math|Transform|BreakTransform _output_get))) 0.5))))) (.Y (Math|Vector|BreakVector (+ (.Location (Math|Transform|BreakTransform _output_get)) (Math|Transform|TransformLocation (Math|Transform|MakeTransform "0, 0, 0" (.Rotation (Math|Transform|BreakTransform _output_get))) (* (- (Math|Vector|MakeVector (* (.X (Utilities|Struct|BreakIntPoint _output_get_3)) (.X (Math|Vector|BreakVector (.Scale (Math|Transform|BreakTransform _output_get))))) (* (.Y (Utilities|Struct|BreakIntPoint _output_get_3)) (.Y (Math|Vector|BreakVector (.Scale (Math|Transform|BreakTransform _output_get))))) 0.512) (.Scale (Math|Transform|BreakTransform _output_get))) 0.5))))) 5e+04) false false)
      (Transformation|SetActorRotation (Math|Rotator|MakeRotator 0.0 0.0 (.Yaw (Math|Rotator|BreakRotator (.Rotation (Math|Transform|BreakTransform _output_get))))))
      (Utilities|InitRTs))))

(fn ConstructionScript
  (bind _scenecapturecomponent2d (Variables|Default|GetSceneCaptureComponent2D))
  (Variables|Default|SetUpdateNeeded! false)
  (Utilities|FlowControl|Sequence
    (:then_0
      (Utilities|InitZOffset)
      (Utilities|InitRTs))
    (:then_1
      (if (Variables|Selection|GetSalectAllRoads!)
        (CallFunction|SelectAllRoads)
        (else
          (for _array_element (Variables|Selection|GetSelectedRoads)
            (Rendering|SceneCapture|ShowOnlyActorComponents _scenecapturecomponent2d (Utilities|ResolveSoftReference _array_element) false)
            (Class|SceneCaptureComponent|HideActorComponents _scenecapturecomponent2d (Utilities|ResolveSoftReference (stale _array_element_2)) false))
          (for _array_element_2 (Variables|Selection|GetExcludedRoads)
            (Class|SceneCaptureComponent|HideActorComponents _scenecapturecomponent2d (Utilities|ResolveSoftReference _array_element_2) false)))))))

(fn Render
  (params (InIsHeightmap :type Boolean) (InCombinedResult :type Texture%20Render%20Target%202D%20Object%20Reference) (InWeightmapLayerName :type Name%20%28by%20ref%29 :default "None"))
  (bind _depth_rt (Variables|Debug|RTs|GetDepth_RT))
  (bind _heightmap_rt (Variables|Debug|RTs|GetHeightmap_RT))
  (bind _cache_df_rt (Variables|Debug|RTs|GetCache_DF_RT))
  (bind _lsrtsize (Variables|Debug|GetLSRTSize))
  (bind _weightmap_rt (Variables|Debug|RTs|GetWeightmap_RT))
  (bind (_x _y) (Utilities|Struct|BreakIntPoint _lsrtsize))
  (Utilities|Array|AddUnique (Variables|Default|GetAffectedWeightmapLayers) (Variables|BrushSettings|PaintLayers|GetPaintLayerName))
  (if InIsHeightmap
    (Variables|Debug|RTs|SetHeightmap_RT_B InCombinedResult)
    (Rendering|ClearRenderTarget2D _heightmap_rt)
    ;[1 1 1] CaptureRoadsHeightmap
    (Development|ExecuteConsoleCommand "r.forcelod 0" 0)
    (Rendering|SceneCapture|CaptureScene (Variables|Default|GetSceneCaptureComponent2D) :!class /Script/Engine.SceneCaptureComponent2D)
    (Development|ExecuteConsoleCommand "r.forcelod -1" 0)
    ;[1 1 1] JumpFlood
    (Utilities|IsValid _depth_rt
      (:Is%20Valid
        (Default|JumpFlood :self (Variables|Default|GetJumpFlood_Component2D1) :SeedRT _depth_rt :SceneCaptureZ 5e+04 :UseDepth true :Z%20Location (Variables|Falloff|GetZOffset)))
      (:Is%20Not%20Valid
        _))
    ;[1 1 1] Cache DF to 8RG RT
    (Rendering|ClearRenderTarget2D _cache_df_rt)
    (bind _returnvalue (Rendering|Material|CreateDynamicMaterialInstance "/Game/SnappyRoads/Blueprints/BlueprintBrushes/M_SR_CacheDistanceField_RG8.M_SR_CacheDistanceField_RG8" "None" "None" :!class /Script/Engine.KismetMaterialLibrary))
    (Rendering|Material|SetTextureParameterValue _returnvalue "JumpFloodRT" (select (== (Math|Integer|%(Integer) (Math|Float|Ceil (Math|Float|Log (Math|Conversions|ToFloat(Integer) (Math|Integer|Max(Integer) _x _y)) 2.0)) 2) 0) (Variables|Debug|RTs|GetJF_RT_A) (Variables|Debug|RTs|GetJF_RT_B)))
    (Rendering|Material|SetScalarParameterValue _returnvalue "UseBlur" 1.0 :!class /Script/Engine.MaterialInstanceDynamic)
    (Rendering|Material|SetScalarParameterValue _returnvalue "Bluroffset" (Variables|Effects|GetRoadShapeBlur) :!class /Script/Engine.MaterialInstanceDynamic)
    (Rendering|DrawMaterialtoRenderTarget _cache_df_rt _returnvalue)
    ;[1 1 1] Draw 32R Depth to  8RG Heightmap RT
    (bind _returnvalue_2 (Rendering|Material|CreateDynamicMaterialInstance "/Game/SnappyRoads/Blueprints/BlueprintBrushes/M_SR_SimpleBrush.M_SR_SimpleBrush" "None" "None" :!class /Script/Engine.KismetMaterialLibrary))
    (Rendering|Material|SetTextureParameterValue _returnvalue_2 "HeightRT" InCombinedResult)
    (Rendering|Material|SetTextureParameterValue _returnvalue_2 "DepthRT" (Variables|Debug|RTs|GetDepth_RT))
    (Rendering|Material|SetTextureParameterValue _returnvalue_2 "CacheRT" (Variables|Debug|RTs|GetCache_DF_RT))
    (Rendering|Material|SetScalarParameterValue _returnvalue_2 "ZOffset" (Variables|Falloff|GetZOffset) :!class /Script/Engine.MaterialInstanceDynamic)
    (Rendering|Material|SetScalarParameterValue _returnvalue "FallofWidth" (Variables|Falloff|GetRoadFallofWidth) :!class /Script/Engine.MaterialInstanceDynamic)
    (Rendering|Material|SetScalarParameterValue _returnvalue "TrenchOffset" (Variables|Falloff|GetTrenchOffset) :!class /Script/Engine.MaterialInstanceDynamic)
    (Rendering|Material|SetScalarParameterValue _returnvalue_2 "TrenchDepth" (Variables|Falloff|GetTrenchDepthMultiplier) :!class /Script/Engine.MaterialInstanceDynamic)
    (Rendering|Material|SetScalarParameterValue _returnvalue_2 "BlendMode" (Math|Conversions|ToFloat(Byte) (Variables|BrushSettings|GetBrushBlendMode)) :!class /Script/Engine.MaterialInstanceDynamic)
    (Rendering|DrawMaterialtoRenderTarget _heightmap_rt _returnvalue_2)
    (else
      ;[1 1 1] PaintLayer
      (Rendering|ClearRenderTarget2D _weightmap_rt)
      (bind _returnvalue_3 (Rendering|Material|CreateDynamicMaterialInstance "/Game/SnappyRoads/Blueprints/BlueprintBrushes/M_SR_SimpleBrush.M_SR_SimpleBrush" "None" "None" :!class /Script/Engine.KismetMaterialLibrary))
      (Rendering|Material|SetTextureParameterValue _returnvalue_3 "HeightRT" InCombinedResult)
      (Rendering|Material|SetTextureParameterValue _returnvalue_3 "DepthRT" (Variables|Debug|RTs|GetDepth_RT))
      (Rendering|Material|SetTextureParameterValue _returnvalue_3 "CacheRT" (Variables|Debug|RTs|GetCache_DF_RT))
      (Rendering|Material|SetTextureParameterValue _returnvalue_3 "HeightmapRT" (Variables|Debug|RTs|GetHeightmap_RT_B))
      (Rendering|Material|SetScalarParameterValue _returnvalue_3 "ZOffset" (Variables|Falloff|GetZOffset) :!class /Script/Engine.MaterialInstanceDynamic)
      (Rendering|Material|SetScalarParameterValue _returnvalue_3 "Paint" 1.0 :!class /Script/Engine.MaterialInstanceDynamic)
      (Rendering|Material|SetScalarParameterValue _returnvalue_3 "PaintClipHeight" (Variables|BrushSettings|PaintLayers|GetPaintClipHeight) :!class /Script/Engine.MaterialInstanceDynamic)
      (Rendering|Material|SetScalarParameterValue _returnvalue_3 "PaintFalloffWidth" (Variables|BrushSettings|PaintLayers|GetPaintFalloffWidth) :!class /Script/Engine.MaterialInstanceDynamic)
      (Rendering|Material|SetScalarParameterValue _returnvalue_3 "PaintFalloffOffset" (Variables|BrushSettings|PaintLayers|GetPaintFalloffOffset) :!class /Script/Engine.MaterialInstanceDynamic)
      (Rendering|DrawMaterialtoRenderTarget _weightmap_rt _returnvalue_3)))
  (return (select InIsHeightmap (Variables|Debug|RTs|GetHeightmap_RT) (Variables|Debug|RTs|GetWeightmap_RT))))