(event Custom|Build
  (bind _returnvalue (Transformation|GetActorScale3D))
  (bind _网格体 (Variables|连接处|Get网格体))
  (bind (_lenght _width) (Utilities|GetMeshLength _网格体))
  (Utilities|FlowControl|Sequence
    (:then_0
      ;[1 1 1] Add intersection static mesh
      (bind _网格体_2 (Variables|连接处|Get网格体)
        (:then
          (bind _returnvalue_2 (AddComponent|AddStaticMeshComponent false (Math|Transform|MakeTransform "0, 0, 0" "0, 0, 0" (Variables|连接处|Get缩放))))
          (bind _output_get (Variables|Core|SetIntersectionMeshComp _returnvalue_2))
          (Variables|/Script/Engine.ActorComponent|SetComponentTags _returnvalue_2 (Utilities|Array|MakeArray "Intersection"))
          (bind _target (Utilities|SetMeshConfig _output_get _网格体_2))
          (Utilities|SetMaterialOverrides _target 0.0 0.0))
        (:else)))
    (:then_1
      ;[1 1 1] WIP, Add intersection corners (resizable intersection)
      (CallFunction|AddIntersectionCorners))
    (:then_2
      ;[1 1 1] CornerExtra. Adds extra meshes at corners of the bounding box
      (for _array_element (Variables|连接处|Get边界扩展)
        (bind _returnvalue_3 (Utilities|SampleCorners (Variables|连接处|Get网格体) (.Offset (Utilities|Struct|BreakFMeshExtraSettings _array_element)) (.RotationZ (Utilities|Struct|BreakFMeshExtraSettings _array_element))))
        (bind _returnvalue_4 (Game|AddComponentbyClass "/Script/Engine.HierarchicalInstancedStaticMeshComponent" true))
        (Utilities|SetMeshConfig _returnvalue_4 (.Mesh (Utilities|Struct|BreakFMeshExtraSettings _array_element)))
        (Components|InstancedStaticMesh|AddInstances _returnvalue_4 _returnvalue_3 false false)
        ;;[1 1 1] Don't scale mesh extra
        (Transformation|AttachComponentToComponent _returnvalue_4 (Variables|Default|GetDefaultSceneRoot) "None" "KeepRelative" "KeepRelative" "KeepWorld" true)))
    (:then_3
      ;[1 1 1] WIP MeshExtra. Adds a single mesh at the center
      (for _array_element_2 (Variables|连接处|Get网格体扩展)
        (bind _returnvalue_5 (Game|AddComponentbyClass "/Script/Engine.StaticMeshComponent" true))
        (Utilities|SetMeshConfig _returnvalue_5 (.Mesh (Utilities|Struct|BreakFMeshExtraSettings _array_element_2)))
        ;;[1 1 1] Don't scale mesh extra
        (Transformation|AttachComponentToComponent _returnvalue_5 (Variables|Default|GetDefaultSceneRoot) "None" "KeepRelative" "KeepRelative" "KeepWorld" true)))
    (:then_4
      ;[1 1 1] To-Do: Add turn 90 deg option
      ; WIP Spline extra (static mesh)
      (for _array_element_3 (Variables|连接处|Get样条扩展)
        (bind _returnvalue_6 (Game|AddComponentbyClass "/Script/Engine.StaticMeshComponent" true (Math|Transform|MakeTransform (+ (Math|Vector|MakeVector 0.0 (.X (Math|Vector2D|BreakVector2D (.Offset (Utilities|Struct|BreakFSplineMeshStettings _array_element_3)))) (.Y (Math|Vector2D|BreakVector2D (.Offset (Utilities|Struct|BreakFSplineMeshStettings _array_element_3))))) (Math|Vector|MakeVector (.x (.Min (Components|StaticMesh|GetLocalBounds (Variables|Core|GetIntersectionMeshComp)))) (Math|Float|SelectFloat (.y (.Max (Components|StaticMesh|GetLocalBounds (Variables|Core|GetIntersectionMeshComp)))) 0.0 (.AnchorRight (Utilities|Struct|BreakFSplineMeshStettings _array_element_3))) 0.0)) "0, 0, 0" (Math|Vector|MakeVector (/ (* _lenght (.x _returnvalue)) (.Lenght (Utilities|GetMeshLength (Utilities|Array|Get(acopy) (.Meshes (Utilities|Struct|BreakFSplineMeshStettings _array_element_3)))))) (Math|Float|SelectFloat (/ (* _width (.y _returnvalue)) (.Width (Utilities|GetMeshLength (Utilities|Array|Get(acopy) (.Meshes (Utilities|Struct|BreakFSplineMeshStettings _array_element_3)))))) 1.0 (.UseScale (Utilities|Struct|BreakFSplineMeshStettings _array_element_3))) 1.0))))
        (Components|StaticMesh|SetStaticMesh _returnvalue_6 (Utilities|Array|Get(acopy) (.Meshes (Utilities|Struct|BreakFSplineMeshStettings _array_element_3))))
        (Transformation|AttachComponentToComponent _returnvalue_6 (Variables|Default|GetDefaultSceneRoot) "None" "KeepRelative" "KeepRelative" "KeepWorld" true)
        (if (.Mirror (Utilities|Struct|BreakFSplineMeshStettings _array_element_3)) ; Mirror?
          (bind _returnvalue_7 (Game|AddComponentbyClass "/Script/Engine.StaticMeshComponent" true (Math|Transform|MakeTransform (* (+ (Math|Vector|MakeVector 0.0 (.X (Math|Vector2D|BreakVector2D (.Offset (Utilities|Struct|BreakFSplineMeshStettings _array_element_3)))) (.Y (Math|Vector2D|BreakVector2D (.Offset (Utilities|Struct|BreakFSplineMeshStettings _array_element_3))))) (Math|Vector|MakeVector (.x (.Min (Components|StaticMesh|GetLocalBounds (Variables|Core|GetIntersectionMeshComp)))) (Math|Float|SelectFloat (.y (.Max (Components|StaticMesh|GetLocalBounds (Variables|Core|GetIntersectionMeshComp)))) 0.0 (.AnchorRight (Utilities|Struct|BreakFSplineMeshStettings _array_element_3))) 0.0)) "1.000000,-1.000000,1.000000") "0, 0, 0" (Math|Vector|MakeVector (/ (* _lenght (.x _returnvalue)) (.Lenght (Utilities|GetMeshLength (Utilities|Array|Get(acopy) (.Meshes (Utilities|Struct|BreakFSplineMeshStettings _array_element_3)))))) (- 0.0 (Math|Float|SelectFloat (/ (* _width (.y _returnvalue)) (.Width (Utilities|GetMeshLength (Utilities|Array|Get(acopy) (.Meshes (Utilities|Struct|BreakFSplineMeshStettings _array_element_3)))))) 1.0 (.UseScale (Utilities|Struct|BreakFSplineMeshStettings _array_element_3)))) 1.0))))
          (Components|StaticMesh|SetStaticMesh _returnvalue_7 (Utilities|Array|Get(acopy) (.Meshes (Utilities|Struct|BreakFSplineMeshStettings _array_element_3))))
          (Transformation|AttachComponentToComponent _returnvalue_7 (Variables|Default|GetDefaultSceneRoot) "None" "KeepRelative" "KeepRelative" "KeepWorld" true))))))

(fn ConstructionScript
  (bind _returnvalue (Transformation|GetActorTransform))
  (Variables|Core|SetbBaked false)
  (Variables|Core|SetbDeformedLandscape false)
  (Utilities|FlowControl|Sequence
    (:then_0
      ;[1 1 1] Debug
      (Utilities|String|LogString (Utilities|String|Append (Utilities|GetDisplayName self) "::" "Constructor") false))
    (:then_1
      (CallFunction|Build))
    (:then_2
      (if (Variables|连接处|GetbUpdateConnectedRoads)
        (Default|CallOnChanged)))
    (:then_3
      ;[1 1 1] Reset transform fix
      (if (and (== _returnvalue (Math|Transform|MakeTransform "0, 0, 0" "0, 0, 0" "1.000000,1.000000,1.000000")) (not (== (Variables|Core|Get最后变换) (Math|Transform|MakeTransform "0, 0, 0" "0, 0, 0" "1.000000,1.000000,1.000000"))))
        (Transformation|SetActorTransform (Variables|Core|Get最后变换))
        (Utilities|String|LogString (Utilities|String|Append (Utilities|GetDisplayName self) ": Prevented transform from resetting! " (Utilities|String|ToString(Transform) (Variables|Core|Get最后变换))))
        (else
          (Variables|Core|Set最后变换 _returnvalue))))))

(fn Connect
  (params (AutoUpdateTangents :type Boolean))
  (bind _returnvalue (Transformation|GetActorTransform))
  (bind _连接到 (Variables|连接|Get连接到))
  (bind _连接到_2 (Variables|连接|Get连接到))
  (bind _连接模板 (Variables|连接|Get连接模板))
  (bind _output (Utilities|ResolveSoftReference _连接模板))
  (bind _output_2 (Utilities|ResolveSoftReference _连接到_2))
  (Utilities|IsValid _output_2
    (:Is%20Valid
      (Utilities|FlowControl|Sequence
        (:then_0
          ;[1 1 1] Spawn a Road
          (bind _returnvalue_2 (Game|SpawnActorfromClass "/Game/SnappyRoads/Blueprints/BP_SnappyRoad.BP_SnappyRoad_C" (Math|Transform|MakeTransform (.location _returnvalue) (.rotation _returnvalue) "1.000000,1.000000,1.000000") "Undefined" 0 0))
          (bind _output_get (LocalVariables|SetRoad_ _returnvalue_2))
          (Variables|/Game/SnappyRoads/Blueprints/BP_SnappyRoad.BP_SnappyRoad_C|Set自动更新切线 _output_get AutoUpdateTangents)
          (Utilities|IsValid _output
            (:Is%20Valid
              (Default|CopyConfig _output _output_get 0 false false true)
              (Default|ClearSplineMeshes _output_get))
            (:Is%20Not%20Valid
              (bind _oppositeroad (连接|FindMostOppositeRoad (- (Transformation|GetActorLocation _output_2) (.location _returnvalue)) (Utilities|Array|MakeArray _output_get)))
              (Utilities|IsValid _oppositeroad
                (:Is%20Valid
                  (Default|CopyConfig _oppositeroad _output_get 0 false false true)
                  (Default|ClearSplineMeshes _output_get)
                  (Utilities|String|LogString (Utilities|String|Append "Found: " (Utilities|GetDisplayName _oppositeroad))))
                (:Is%20Not%20Valid
                  (Utilities|String|LogString "NotFound"))))))
        (:then_1
          ;[1 1 1] Set Connected Intersections
          (Utilities|Struct|SetmembersinFConnection (Variables|/Game/SnappyRoads/Blueprints/BP_SnappyRoad.BP_SnappyRoad_C|Get开始时链接 (LocalVariables|GetRoad_)) (Utilities|ResolveSoftReference self) "None")
          (Utilities|Struct|SetmembersinFConnection (Variables|/Game/SnappyRoads/Blueprints/BP_SnappyRoad.BP_SnappyRoad_C|Get结束时链接 (LocalVariables|GetRoad_)) _连接到 "None")
          (Spline|SetLocationatSplinePoint (Variables|/Game/SnappyRoads/Blueprints/BP_SnappyRoad.BP_SnappyRoad_C|GetSpline (LocalVariables|GetRoad_)) 1 (Transformation|GetActorLocation (Utilities|ResolveSoftReference _连接到)) "World" false))
        (:then_2
          ;[1 1 1] Update
          (Default|BindonIntersectionChanged (LocalVariables|GetRoad_))
          (Default|UpdateTangents (LocalVariables|GetRoad_)) ; Update & Rebuild
        )
        (:then_3
          (return (LocalVariables|GetRoad_)))))))

(fn AddIntersectionCorners
  (bind _corner (Variables|连接处|GetCorner)
    (:then
      (bind (_meshout _returnvalue) (Utilities|SampleCorners _corner (Variables|连接处|GetCornerOffset) 0.0))
      (for _array_element _returnvalue
        (bind _returnvalue_2 (Game|AddComponentbyClass "/Script/Engine.StaticMeshComponent" true _array_element))
        (Utilities|Array|Add (LocalVariables|Get_Comp) _returnvalue_2)
        (Components|StaticMesh|SetStaticMesh _returnvalue_2 _meshout)
        ;[1 1 1] Don't scale
        (Transformation|AttachComponentToComponent _returnvalue_2 (Variables|Default|GetDefaultSceneRoot) "None" "KeepRelative" "KeepRelative" "KeepWorld" true)))
    (:else)))

(fn SampleCorners
  (params (Mesh :type Static%20Mesh%20Object%20Reference) (Offset :type Vector) (Rotation%20Z%20%28Yaw%29 :type Float%20%28double-precision%29) (Component :type Primitive%20Component%20Object%20Reference))
  (bind _returnvalue (StaticMesh|GetBounds Mesh))
  (for _index (range 0 3)
    (Utilities|Array|Add (LocalVariables|GetPoints) (Math|Transform|ComposeTransforms (Math|Transform|MakeTransform Offset (Math|Rotator|MakeRotator 0.0 0.0 Rotation%20Z%20%28Yaw%29)) (Math|Transform|MakeTransform (+ (* (.origin _returnvalue) "1.000000,1.000000, 0") (* (* (.boxextent _returnvalue) (Variables|连接处|Get缩放)) (Utilities|Array|Get(acopy) (Utilities|Array|MakeArray "1.000000,1.000000, 0" "-1.000000,1.000000,0.000000" "-1.000000,-1.000000,0.000000" "1.000000,-1.000000, 0") _index))) (Math|Rotator|MakeRotator 0.0 0.0 (Math|Conversions|ToFloat(Integer) (* _index 90)))))))
  (return Mesh (LocalVariables|GetPoints)))

(fn 对齐地面
  (bind _returnvalue (Transformation|GetActorLocation))
  (bind _outhits (Class|KismetSystemLibrary|LineTraceMultiforObjects _returnvalue (+ _returnvalue "0, 0,-5000.000000") (Utilities|Array|MakeArray "ObjectTypeQuery1") false 0 "ForOneFrame" true))
  (for _array_element _outhits
    (Utilities|Casting|CastToLandscape (.HitActor (Collision|BreakHitResult _array_element)))
    (Transformation|SetActorLocation (+ (.Location (Collision|BreakHitResult _array_element)) "0, 0,10.000000") false false))
  (Default|CallOnChanged))

(fn 删除
  (Actor|DestroyActor))

(fn SpawnConnectedRoads
  (bind _intersectionmeshcomp (Variables|Core|GetIntersectionMeshComp)
    (:then
      (for _array_element (Transformation|GetAllSocketNames _intersectionmeshcomp)
        (bind _returnvalue (Collision|SphereOverlapActors (.location (Transformation|GetSocketTransform _intersectionmeshcomp _array_element "RTS_World")) 1e+02 (Utilities|Array|MakeArray "ObjectTypeQuery1") "/Game/SnappyRoads/Blueprints/BP_SnappyRoad.BP_SnappyRoad_C"))
        (if (not _returnvalue)
          (bind _returnvalue_2 (Game|SpawnActorfromClass "/Game/SnappyRoads/Blueprints/BP_SnappyRoad.BP_SnappyRoad_C" (Math|Transform|MakeTransform (.location (Transformation|GetSocketTransform _intersectionmeshcomp _array_element "RTS_World")) (.rotation (Transformation|GetSocketTransform _intersectionmeshcomp _array_element "RTS_World")) "1.000000,1.000000,1.000000") "Undefined" 0 0))
          (Utilities|Struct|SetmembersinFConnection (Variables|/Game/SnappyRoads/Blueprints/BP_SnappyRoad.BP_SnappyRoad_C|Get开始时链接 _returnvalue_2) (Utilities|ResolveSoftReference self) _array_element)
          (Default|BindonIntersectionChanged _returnvalue_2))))
    (:else)))

(fn DisconnectAll
  (bind _self self)
  (EventDispatchers|UnbindallEventsfromOnChanged)
  (bind _connectedroads (连接|FindConnectedRoads))
  (for _array_element _connectedroads
    (Default|UnbindonIntersectionChanged _array_element)
    (if (== (Utilities|ResolveSoftReference (.Actor (Utilities|Struct|BreakFConnection (Variables|/Game/SnappyRoads/Blueprints/BP_SnappyRoad.BP_SnappyRoad_C|Get结束时链接 _array_element)))) _self)
      (Utilities|Struct|SetmembersinFConnection (Variables|/Game/SnappyRoads/Blueprints/BP_SnappyRoad.BP_SnappyRoad_C|Get结束时链接 _array_element) 0 "None")
      (elif (== _self (Utilities|ResolveSoftReference (.Actor (Utilities|Struct|BreakFConnection (Variables|/Game/SnappyRoads/Blueprints/BP_SnappyRoad.BP_SnappyRoad_C|Get开始时链接 _array_element)))))
        (Utilities|Struct|SetmembersinFConnection (Variables|/Game/SnappyRoads/Blueprints/BP_SnappyRoad.BP_SnappyRoad_C|Get开始时链接 _array_element) 0 "None")))))

(fn Level
  ;[1 1 1] Helper: straighten Z-axis
  (Transformation|SetActorRotation (Math|Rotator|MakeRotator 0.0 0.0 (.yaw (Transformation|GetActorRotation))))
  (Default|CallOnChanged))

(fn FindConnectedRoads
  (bind _intersectionmeshcomp (Variables|Core|GetIntersectionMeshComp))
  (Utilities|IsValid _intersectionmeshcomp
    (:Is%20Valid
      (for _array_element (Transformation|GetAllSocketNames _intersectionmeshcomp)
        (bind (_outactors _returnvalue) (Collision|SphereOverlapActors (Transformation|GetSocketLocation _intersectionmeshcomp _array_element) 1e+02 (Utilities|Array|MakeArray "ObjectTypeQuery1") "/Game/SnappyRoads/Blueprints/BP_SnappyRoad.BP_SnappyRoad_C"))
        (if _returnvalue
          (bind _asbp_snappy_road (Utilities|Casting|CastToBP_SnappyRoad (Utilities|Array|Get(acopy) _outactors)))
          (Utilities|Array|AddUnique (LocalVariables|GetConnectedRoads_) _asbp_snappy_road)
          (Utilities|Array|Add (LocalVariables|GetbIsRoadStart_) (Utilities|Operators|EqualEqual (Transformation|GetWorldLocation (Variables|/Game/SnappyRoads/Blueprints/BP_SnappyRoad.BP_SnappyRoad_C|GetRoadStart _asbp_snappy_road)) (Transformation|GetSocketLocation _intersectionmeshcomp _array_element) 5e+01))
          (Utilities|String|LogString (Utilities|GetDisplayName _asbp_snappy_road) false)))
      (return (LocalVariables|GetConnectedRoads_) (LocalVariables|GetbIsRoadStart_)))))

(fn FindMostOppositeRoad
  (params (Direction :type Vector) (ActorsToIgnore :type Array%20of%20Actor%20Object%20References))
  (bind _returnvalue (Math|Rotator|MakeRotfromX Direction))
  (bind _intersectionmeshcomp (Variables|Core|GetIntersectionMeshComp))
  (bind _returnvalue_2 (Transformation|GetSocketTransform _intersectionmeshcomp "None" "RTS_Component"))
  (bind _returnvalue_3 (Math|Rotator|MakeRotfromX (.location _returnvalue_2)))
  (bind _returnvalue_4 (Math|Rotator|Delta(Rotator) _returnvalue _returnvalue_3))
  (bind _returnvalue_5 (Math|Float|Absolute(Float) (.yaw _returnvalue_4)))
  (for _array_element (Transformation|GetAllSocketNames _intersectionmeshcomp)
    (bind (_outactors _returnvalue_6) (Collision|SphereOverlapActors (Transformation|GetSocketLocation _intersectionmeshcomp _array_element) 5e+01 (Utilities|Array|MakeArray "ObjectTypeQuery1" "ObjectTypeQuery2") "/Game/SnappyRoads/Blueprints/BP_SnappyRoad.BP_SnappyRoad_C" ActorsToIgnore))
    (if _returnvalue_6
      (if (< _returnvalue_5 (LocalVariables|GetDeltaMin_))
        (LocalVariables|SetOppositeRoad_ (.AsBP%20Snappy%20Road (Utilities|Casting|CastToBP_SnappyRoad (Utilities|Array|Get(acopy) _outactors))))
        (LocalVariables|SetDeltaMin_ _returnvalue_5))))
  (return (LocalVariables|GetOppositeRoad_)))

(fn 修复连接
  (连接|DisconnectAll)
  (bind _connectedroads (连接|FindConnectedRoads))
  (for _array_element _connectedroads
    (Default|Snap _array_element)))

(fn Connect
  (连接|Connect false))