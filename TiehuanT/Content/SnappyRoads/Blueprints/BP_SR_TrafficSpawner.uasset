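; Traffic spawner for Snappy Roads that populates a spline route with simple vehicles.
; UpdateSplinePath merges the FollowPath actors' splines into one local spline, scaling tangents at junctions by gap length to shape the connections.
; On BeginPlay it spawns BP_SimpleVehicle actors along that spline, cycling meshes and randomizing speed and lane.
; Unless OneWay is set, it flips Reverse and spawns again for oncoming traffic, doubling the vehicle count.
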(event Custom|UpdateSplinePath
  (bind _returnvalue (Transformation|GetActorTransform))
  (bind _spline (Variables|Default|GetSpline))
  (bind _spline_2 (Variables|Default|GetSpline))
  (bind _spline_3 (Variables|Default|GetSpline))
  ;[1 1 1] BuildPathSpline
  (Spline|ClearSplinePoints (Variables|Default|GetSpline) false)
  (Variables|Core|Set_Counter 0)
  (for (_array_element _array_index) (Variables|Default|GetFollowPath)
    (for _index (range 0 (Class|SplineComponent|GetNumberOfSplineSegments (Variables|/Game/SnappyRoads/Blueprints/BP_SnappyRoad.BP_SnappyRoad_C|GetSpline (Utilities|ResolveSoftReference _array_element))))
      (Class|SplineComponent|AddPoint _spline_3 (Utilities|Struct|MakeSplinePoint (Math|Conversions|ToFloat(Integer) (Variables|Core|Get_Counter)) (Math|Transform|InverseTransformLocation _returnvalue (.Location (Spline|GetLocationandTangentatSplinePoint (Variables|/Game/SnappyRoads/Blueprints/BP_SnappyRoad.BP_SnappyRoad_C|GetSpline (Utilities|ResolveSoftReference _array_element)) _index "World"))) (Math|Vector|SelectVector (* (Math|Vector|Normalize (Math|Transform|InverseTransformDirection _returnvalue (Spline|GetArriveTangentatSplinePoint (Variables|/Game/SnappyRoads/Blueprints/BP_SnappyRoad.BP_SnappyRoad_C|GetSpline (Utilities|ResolveSoftReference _array_element)) _index "World"))) (Math|Vector|VectorLength (- (Math|Transform|InverseTransformLocation _returnvalue (.Location (Spline|GetLocationandTangentatSplinePoint (Variables|/Game/SnappyRoads/Blueprints/BP_SnappyRoad.BP_SnappyRoad_C|GetSpline (Utilities|ResolveSoftReference _array_element)) _index "World"))) (Math|Transform|InverseTransformLocation _returnvalue (.Location (Spline|GetLocationandTangentatSplinePoint _spline_2 (- (Variables|Core|Get_Counter) 1) "World")))))) (Math|Transform|InverseTransformDirection _returnvalue (Spline|GetArriveTangentatSplinePoint (Variables|/Game/SnappyRoads/Blueprints/BP_SnappyRoad.BP_SnappyRoad_C|GetSpline (Utilities|ResolveSoftReference _array_element)) _index "World")) (== _index 0)) (Math|Transform|InverseTransformDirection _returnvalue (.Tangent (Spline|GetLocationandTangentatSplinePoint (Variables|/Game/SnappyRoads/Blueprints/BP_SnappyRoad.BP_SnappyRoad_C|GetSpline (Utilities|ResolveSoftReference _array_element)) _index "World"))) "0.000000,0.000000,0.000000" "1.000000,1.000000,1.000000" "CurveCustomTangent") false)
      (Class|SplineComponent|SetUpVectoratSplinePoint _spline_3 (Class|SplineComponent|GetNumberOfSplineSegments _spline_3) (Class|SplineComponent|GetUpVectoratSplinePoint (Variables|/Game/SnappyRoads/Blueprints/BP_SnappyRoad.BP_SnappyRoad_C|GetSpline (Utilities|ResolveSoftReference _array_element)) _index "World") "World" true)
      ;;[1 1 1] Scale tangents at intersection
      (if (and (== _index 0) (> _array_index 0))
        (Spline|UpdateSpline _spline)
        (Spline|SetTangentsatSplinePoint _spline (- (Variables|Core|Get_Counter) 1) (Math|Transform|InverseTransformDirection _returnvalue (Spline|GetArriveTangentatSplinePoint _spline_2 (- (Variables|Core|Get_Counter) 1) "World")) (* (Math|Vector|Normalize (Math|Transform|InverseTransformDirection _returnvalue (.Tangent (Spline|GetLocationandTangentatSplinePoint _spline_2 (- (Variables|Core|Get_Counter) 1) "World")))) (Math|Vector|VectorLength (- (Math|Transform|InverseTransformLocation _returnvalue (.Location (Spline|GetLocationandTangentatSplinePoint (Variables|/Game/SnappyRoads/Blueprints/BP_SnappyRoad.BP_SnappyRoad_C|GetSpline (Utilities|ResolveSoftReference _array_element)) _index "World"))) (Math|Transform|InverseTransformLocation _returnvalue (.Location (Spline|GetLocationandTangentatSplinePoint _spline_2 (- (Variables|Core|Get_Counter) 1) "World")))))) "Local" false))
      (Math|Integer|IncrementInt (Variables|Core|Get_Counter))))
  (Spline|UpdateSpline (Variables|Default|GetSpline)))

(event EventBeginPlay
  (bind _vehiclemeshes (Variables|Default|GetVehicleMeshes))
  (Utilities|FlowControl|Sequence
    (:then_1
      ;[1 1 1] SpawnVehicles
      (for _index (range 1 (Variables|Default|GetVehiclesNum)) :!label _label
        (Game|SpawnActorfromClass "/Game/SnappyRoads/Blueprints/Vehicle/BP_SimpleVehicle.BP_SimpleVehicle_C" (Math|Transform|MakeTransform "0, 0, 0" "0, 0, 0" "1.000000,1.000000,1.000000") "Undefined" 0 (Utilities|Array|Get(acopy) _vehiclemeshes (Math|Integer|%(Integer) _index (Utilities|Array|Length _vehiclemeshes))) (Utilities|Struct|MakeFTrafficConfig (Variables|Default|GetSpline) (Math|Conversions|ToFloat(Integer) (Math|Float|Round (Math|Random|RandomFloatinRange (Variables|Default|GetMinSpeed) (Variables|Default|GetMaxSpeed)))) (Variables|Default|GetVehicleOffset) (Math|Random|RandomIntegerinRange (Variables|Default|GetMinLane) (Variables|Default|GetMaxLane)) (Variables|Default|GetLaneWidth) (Variables|Default|GetVehicleRotation) (Variables|Default|GetReverse)) (Variables|Default|GetUseRandomColor) 0)))
    (:then_2
      ;[1 1 1] RepeatForOncomingTraffic
      ; So we have double the amount of vehicles specified!
      (if (not (Variables|Default|GetOneWay))
        (Variables|Default|SetReverse (not (Variables|Default|GetReverse)))
        (goto _label)))))

(fn ConstructionScript)