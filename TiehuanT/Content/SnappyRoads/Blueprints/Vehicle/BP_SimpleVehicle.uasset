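; BP_SimpleVehicle is a traffic vehicle that follows a spline lane through BPFollowPathComponent.
; Its construction script applies config for direction, jittered lane offset, mesh, speed and optional random color, and places the headlight decal and sensor sphere ahead.
; Sphere overlaps stop it for other pawns or halted vehicles, relay braking via the OnBreak dispatcher, and pass higher speeds to the vehicle ahead.
; Ending the overlap re-enables movement.
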(event OnComponentBeginOverlap(Sphere)
  (params (OverlappedComponent :type Primitive%20Component%20Object%20Reference) (OtherActor :type Actor%20Object%20Reference) (OtherComp :type Primitive%20Component%20Object%20Reference) (OtherBodyIndex :type Integer) (bFromSweep :type Boolean) (SweepResult :type Hit%20Result%20Structure%20%28by%20ref%29))
  (bind _bp_followpath_component (Variables|Default|GetBP_FollowPath_Component))
  (bind _bp_followpath_component_2 (Variables|Default|GetBP_FollowPath_Component))
  ;[1 1 1] Condition
  (Utilities|IsValid (Variables|Core|GetCollidingVehicle)
    (:Is%20Not%20Valid
      (bind _asbp_simple_vehicle (Utilities|Casting|CastToBP_SimpleVehicle OtherActor)
        (:then
          (if true
            ;[1 1 1] Break & SwapSpeeds
            (Utilities|FlowControl|Sequence
              (:then_0
                (Variables|Core|SetCollidingVehicle _asbp_simple_vehicle)
                (Variables|Core|SetbDrawDebug true)
                (EventDispatchers|AssignOnBreak _asbp_simple_vehicle (delegate Custom|OnBreak_Event)))
              (:then_1
                (if (not (Class|ActorComponent|IsComponentTickEnabled (Variables|BP_SimpleVehicle_C|GetBP_FollowPath_Component _asbp_simple_vehicle)))
                  (Variables|/Game/SnappyRoads/Blueprints/Core/Components/BP_FollowPath_Component.BP_FollowPath_Component_C|SetCurrentSpeed _bp_followpath_component 0.0)
                  (Components|Tick|SetComponentTickEnabled _bp_followpath_component false)
                  (Default|CallOnBreak)))
              (:then_2
                (CallFunction|SwapSpeedValues)))))
        (:CastFailed
          ;[1 1 1] PawnCollision
          (Utilities|Casting|CastToPawn OtherActor)
          (Variables|/Game/SnappyRoads/Blueprints/Core/Components/BP_FollowPath_Component.BP_FollowPath_Component_C|SetCurrentSpeed _bp_followpath_component_2 0.0)
          (Components|Tick|SetComponentTickEnabled _bp_followpath_component_2 false)
          (Default|CallOnBreak)
          (Utilities|IsValid (Variables|Core|GetCollidingVehicle)
            (:Is%20Valid
              (EventDispatchers|UnbindEventfromOnBreak (Variables|Core|GetCollidingVehicle) (delegate Custom|OnBreak_Event))
              (Variables|Core|SetCollidingVehicle 0))))))))

(event OnComponentEndOverlap(Sphere)
  (params (OverlappedComponent :type Primitive%20Component%20Object%20Reference) (OtherActor :type Actor%20Object%20Reference) (OtherComp :type Primitive%20Component%20Object%20Reference) (OtherBodyIndex :type Integer))
  (Components|Tick|SetComponentTickEnabled (Variables|Default|GetBP_FollowPath_Component) true)
  (Variables|Core|SetbDrawDebug false)
  (Utilities|IsValid (Variables|Core|GetCollidingVehicle)
    (:Is%20Valid
      (EventDispatchers|UnbindEventfromOnBreak (Variables|Core|GetCollidingVehicle) (delegate Custom|OnBreak_Event))
      (Variables|Core|SetCollidingVehicle 0))))

(event Custom|OnBreak_Event
  (bind _bp_followpath_component (Variables|Default|GetBP_FollowPath_Component))
  ;[1 1 1] PawnCollision
  (Variables|/Game/SnappyRoads/Blueprints/Core/Components/BP_FollowPath_Component.BP_FollowPath_Component_C|SetCurrentSpeed _bp_followpath_component 0.0)
  (Components|Tick|SetComponentTickEnabled _bp_followpath_component false)
  (Default|CallOnBreak)
  (Utilities|IsValid (Variables|Core|GetCollidingVehicle)
    (:Is%20Valid
      (EventDispatchers|UnbindEventfromOnBreak (Variables|Core|GetCollidingVehicle) (delegate Custom|OnBreak_Event))
      (Variables|Core|SetCollidingVehicle 0))))

(event EventTick
  (params (DeltaSeconds :type Float%20%28single-precision%29))
  ;[1 1 1] DebugDraw
  (if (Variables|Core|GetbDrawDebug)
    (Rendering|Debug|DrawDebugSphere (Transformation|GetWorldLocation (Variables|Default|GetSphere)) 1e+02 12 "(R=1.000000,G=0.061921,B=0.000000,A=1.000000)" 0.0)
    (Rendering|Debug|DrawDebugArrow (+ (Transformation|GetWorldLocation (stale OnComponentBeginOverlap(Sphere) OverlappedComponent)) "0, 0,300.000000") (+ (Transformation|GetWorldLocation (stale OnComponentBeginOverlap(Sphere) OtherComp)) "0, 0,300.000000") 5e+02 "(R=0.000000,G=1.000000,B=0.127348,A=1.000000)" 0.0 5.0)
    (Rendering|Debug|DrawDebugArrow (+ (Transformation|GetWorldLocation (stale OnComponentBeginOverlap(Sphere) OverlappedComponent)) "0, 0,300.000000") (+ (+ (Transformation|GetWorldLocation (stale OnComponentBeginOverlap(Sphere) OverlappedComponent)) "0, 0,300.000000") (* (Math|Vector|GetForwardVector (Transformation|GetWorldRotation (Variables|Default|GetOffset))) 3e+02)) 5e+02 "(R=1.000000,G=0.823312,B=0.000000,A=1.000000)" 0.0 5.0)))

(fn ConstructionScript
  (bind _returnvalue (Math|Random|RandomFloatinRange -4e+01 4e+01))
  (bind _vehicleconfig (Variables|Config|GetVehicleConfig))
  (bind _bp_followpath_component (Variables|Default|GetBP_FollowPath_Component))
  (bind _vehicleconfig_2 (Variables|Config|GetVehicleConfig))
  (bind _staticmesh (Variables|Default|GetStaticMesh))
  (bind _staticmesh_2 (Variables|Default|GetStaticMesh))
  (bind (_spline _speed _offset _lane _lanewidth _rotation _reverse) (Utilities|Struct|BreakFTrafficConfig _vehicleconfig_2))
  (bind (_spline_2 _speed_2 _offset_2 _lane_2 _lanewidth_2 _rotation_2 _reverse_2) (Utilities|Struct|BreakFTrafficConfig _vehicleconfig))
  (bind _min (Components|StaticMesh|GetLocalBounds _staticmesh_2))
  (bind _returnvalue_2 (* _lane_2 _lanewidth_2))
  (bind _returnvalue_3 (Math|Float|Absolute(Float) (.x _min)))
  (bind _returnvalue_4 (+ _returnvalue_2 _returnvalue))
  (bind _returnvalue_5 (+ _offset_2 (Math|Vector2D|MakeVector2D _returnvalue_4 0.0)))
  (Utilities|FlowControl|Sequence
    (:then_0
      ;[1 1 1] Offsets
      (Transformation|SetRelativeRotation (Variables|Default|GetOffset) (Math|Rotator|MakeRotator 0.0 0.0 (Math|Float|SelectFloat 1.8e+02 0.0 _reverse_2)) false false)
      (Transformation|AddLocalOffset (Variables|Default|GetOffset) (Math|Vector|MakeVector 0.0 (.x _returnvalue_5) (.y _returnvalue_5)) false false)
      ;[1 1 1] MeshCosmetics
      (Transformation|SetRelativeRotation _staticmesh _rotation_2 false false)
      (Components|StaticMesh|SetStaticMesh _staticmesh (Variables|Config|GetVehicleMesh)))
    (:then_1
      ;[1 1 1] Position headlight decal in front of the mesh
      (Transformation|AddRelativeLocation (Variables|Default|GetDecal) (Math|Vector|MakeVector (+ _returnvalue_3 5.5e+02) 0.0 0.0) false false)
      (Transformation|AddRelativeLocation (Variables|Default|GetSphere) (Math|Vector|MakeVector (+ _returnvalue_3 2e+02) 0.0 0.0) false false))
    (:then_2
      ;[1 1 1] SetupMovement
      (Variables|/Game/SnappyRoads/Blueprints/Core/Components/BP_FollowPath_Component.BP_FollowPath_Component_C|SetSpline _bp_followpath_component _spline)
      (Variables|/Game/SnappyRoads/Blueprints/Core/Components/BP_FollowPath_Component.BP_FollowPath_Component_C|SetSpeed _bp_followpath_component _speed)
      (Variables|/Game/SnappyRoads/Blueprints/Core/Components/BP_FollowPath_Component.BP_FollowPath_Component_C|SetOffset _bp_followpath_component (Variables|/Script/Engine.SceneComponent|GetRelativeLocation (Variables|Default|GetOffset)))
      (Variables|/Game/SnappyRoads/Blueprints/Core/Components/BP_FollowPath_Component.BP_FollowPath_Component_C|SetReverse _bp_followpath_component _reverse))
    (:then_3
      (if (Variables|Config|GetbUseRandomColor)
        ;[1 1 1] Randomize color
        (bind _returnvalue_6 (Rendering|Material|CreateDynamicMaterialInstance (Variables|Default|GetStaticMesh) 0 "/Game/SnappyRoads/Meshes/Vehicles/Materials/M_Vehicle001_Random.M_Vehicle001_Random" "None" :!class /Script/Engine.PrimitiveComponent))
        (Rendering|Material|SetScalarParameterValue _returnvalue_6 "Color" (Math|Random|RandomFloat) :!class /Script/Engine.MaterialInstanceDynamic)))))

(fn SwapSpeedValues
  (bind _collidingvehicle (Variables|Core|GetCollidingVehicle))
  (bind _bp_followpath_component (Variables|Default|GetBP_FollowPath_Component))
  (bind _bp_followpath_component_2 (Variables|BP_SimpleVehicle_C|GetBP_FollowPath_Component _collidingvehicle))
  (Utilities|IsValid _collidingvehicle
    (:Is%20Valid
      (if (< (Variables|/Game/SnappyRoads/Blueprints/Core/Components/BP_FollowPath_Component.BP_FollowPath_Component_C|GetSpeed _bp_followpath_component_2) (Variables|/Game/SnappyRoads/Blueprints/Core/Components/BP_FollowPath_Component.BP_FollowPath_Component_C|GetSpeed _bp_followpath_component))
        (bind (_min _max) (Utilities|MinMax (Variables|/Game/SnappyRoads/Blueprints/Core/Components/BP_FollowPath_Component.BP_FollowPath_Component_C|GetSpeed _bp_followpath_component_2) (Variables|/Game/SnappyRoads/Blueprints/Core/Components/BP_FollowPath_Component.BP_FollowPath_Component_C|GetSpeed _bp_followpath_component)))
        (Variables|/Game/SnappyRoads/Blueprints/Core/Components/BP_FollowPath_Component.BP_FollowPath_Component_C|SetSpeed _bp_followpath_component_2 _max)
        (Variables|/Game/SnappyRoads/Blueprints/Core/Components/BP_FollowPath_Component.BP_FollowPath_Component_C|SetSpeed _bp_followpath_component _min)
        (if (> (Math|Float|Absolute(Float) (- (Variables|/Game/SnappyRoads/Blueprints/Core/Components/BP_FollowPath_Component.BP_FollowPath_Component_C|GetCurrentSpeed _bp_followpath_component_2) (Variables|/Game/SnappyRoads/Blueprints/Core/Components/BP_FollowPath_Component.BP_FollowPath_Component_C|GetCurrentSpeed _bp_followpath_component))) 2e+01)
          (Variables|/Game/SnappyRoads/Blueprints/Core/Components/BP_FollowPath_Component.BP_FollowPath_Component_C|SetCurrentSpeed _bp_followpath_component (Variables|/Game/SnappyRoads/Blueprints/Core/Components/BP_FollowPath_Component.BP_FollowPath_Component_C|GetCurrentSpeed _bp_followpath_component_2)))))))