(event EventRun
  (CallFunction|Build))

(fn Build
  (bind _splinemeshsettings (Variables|SplineMesh|GetSplineMeshSettings))
  (bind _bsmoothinterp (Variables|SplineMesh|GetbSmoothInterp))
  (bind (_x _y _z) (Math|Vector|BreakVector (.scale _splinemeshsettings)))
  (bind (_x_2 _y_2) (Math|Vector2D|BreakVector2D (.startendoffset _splinemeshsettings)))
  (bind _returnvalue (not (.anchorright _splinemeshsettings)))
  (bind (_roadsegments _rescale) (CallFunction|DistributeSplineMeshes (.distribution _splinemeshsettings) (.meshes _splinemeshsettings) (Math|Vector2D|MakeVector2D _y _z)))
  (CallFunction|SpawnSplineMeshes _roadsegments (.offset _splinemeshsettings) _x_2 _y_2 (.anchor _splinemeshsettings) (.anchorright _splinemeshsettings) false (.reverse _splinemeshsettings) (.usescale _splinemeshsettings) _returnvalue _bsmoothinterp _rescale)
  (if (.mirror _splinemeshsettings)
    (CallFunction|SpawnSplineMeshes _roadsegments (* (.offset _splinemeshsettings) "(X=-1.000000,Y=1.000000)") _x_2 _y_2 (.anchor _splinemeshsettings) (.anchorright _splinemeshsettings) true (not (.reverse _splinemeshsettings)) (.usescale _splinemeshsettings) _returnvalue _bsmoothinterp _rescale)))

(fn GetMeshLength
  (params (StaticMesh :type Static%20Mesh%20Object%20Reference) (OverrideScaleX :type Float%20%28double-precision%29))
  (return (* (.x (.boxextent (StaticMesh|GetBounds StaticMesh))) 2.0 (select (!= OverrideScaleX 1.0) OverrideScaleX (.X (Math|Vector|BreakVector (Variables|Deprecated|GetRoadScale)))))))

(fn GetMeshT
  (params (StaticMesh :type Static%20Mesh%20Object%20Reference))
  (return (/ (CallFunction|GetMeshLength StaticMesh (.X (Math|Vector|BreakVector (.Scale (Utilities|Struct|BreakFSplineMeshStettings (Variables|SplineMesh|GetSplineMeshSettings)))))) (Utilities|GetSplineLength))))

(fn DistributeSplineMeshes
  (params (Distribution :type EDistributionMethod%20Enum :default "NewEnumerator4") (Meshes :type Array%20of%20Static%20Mesh%20Object%20References) (Scale :type Vector%202D%20Structure :default "(X=1.000000,Y=1.000000)"))
  (bind __roadsegments (LocalVariables|Get_RoadSegments))
  (bind __roadsegments_2 (LocalVariables|Get_RoadSegments))
  (bind _splinemeshsettings (Variables|SplineMesh|GetSplineMeshSettings))
  (bind __counter (LocalVariables|Get_Counter))
  (bind _scale (Utilities|Struct|BreakFSplineMeshStettings _splinemeshsettings))
  (bind _returnvalue (Utilities|Array|LastIndex __roadsegments))
  (bind (_x _y _z) (Math|Vector|BreakVector _scale))
  (bind _returnvalue_2 (Math|Vector2D|MakeVector2D _y _z))
  (bind _returnvalue_3 (select false "" _returnvalue_2))
  ;[1 1 1] Distribution
  (bind _output_get (LocalVariables|Set_Meshes Meshes))
  (Utilities|IsValid (Utilities|Array|Get(acopy) _output_get)
    (:Is%20Valid
      (LocalVariables|Set_Stream (Math|Random|MakeRandomStream (Variables|SplineMesh|GetDistributionRandomSeed)))
      (while (LocalVariables|GetbLoop) ; ForEachRoadSegment
        (Utilities|FlowControl|Sequence
          (:then_0
            ;[1 1 1] 1)Pick a mesh according to the distribution method
            (switch Utilities|FlowControl|Switch|SwitchonEDistributionMethod Distribution
              (:NewEnumerator4
                ;[1 1 1] Single
                (LocalVariables|Set_CurrentMesh (Utilities|Array|Get(acopy) (LocalVariables|Get_Meshes))))
              (:NewEnumerator0
                ;[1 1 1] Random
                (LocalVariables|Set_CurrentMesh (Utilities|Array|Get(acopy) (LocalVariables|Get_Meshes) (Class|KismetMathLibrary|RandomIntegerfromStream (Utilities|Array|Length Meshes) (LocalVariables|Get_Stream)))))
              (:NewEnumerator1
                ;[1 1 1] Sequential
                (LocalVariables|Set_CurrentMesh (Utilities|Array|Get(acopy) Meshes (Math|Integer|%(Integer) (LocalVariables|Get_Counter) (Utilities|Array|Length Meshes)))))
              (:NewEnumerator2
                ;[1 1 1] FirstAndLast(FirstMesh)
                (if (>= (Utilities|Array|Length (LocalVariables|Get_Meshes)) 2) ; Do we have 2+ meshes?
                  (if (== (Utilities|Array|Length (LocalVariables|Get_RoadSegments)) 0) ; FirstSegment?
                    ;;[1 1 1] AddLastMeshT in the beggining
                    (LocalVariables|Set_LastMeshT (CallFunction|GetMeshT (Utilities|Array|Get(acopy) (LocalVariables|Get_Meshes) (Utilities|Array|LastIndex (LocalVariables|Get_Meshes)))))
                    (LocalVariables|Set_CurrentMesh (Utilities|Array|Get(acopy) (LocalVariables|Get_Meshes) 1))
                    (else
                      (LocalVariables|Set_CurrentMesh (Utilities|Array|Get(acopy) (LocalVariables|Get_Meshes)) :!label _label)))
                  (else
                    (goto _label))))))
          (:then_1
            ;[1 1 1] 2) Replace (override currently picked mesh)
            (for _array_element (Variables|Core|GetReplaceSegments)
              (if (and (>= __counter (.section _array_element)) (< __counter (+ (.section _array_element) (.repeat _array_element))))
                (LocalVariables|Set_CurrentMesh (.replacewithmesh _array_element)))))
          (:then_2
            ;[1 1 1] Finished?
            (if (or (and (>= _returnvalue 0) (< (- 1.0 (+ (LocalVariables|Get_T) (LocalVariables|Get_LastMeshT))) (- (+ (+ (LocalVariables|Get_T) (LocalVariables|Get_LastMeshT)) (CallFunction|GetMeshT (LocalVariables|Get_CurrentMesh))) 1.0))) (> _returnvalue (Variables|SplineMesh|GetMaxMeshesPerSpline))) ; Finished?
              ;[1 1 1] EndOfSpline
              (LocalVariables|SetbLoop false)
              ;[1 1 1] FirstAndLast(ReplaceFinalSegmentWithLastMesh)
              (if (> (LocalVariables|Get_LastMeshT) 0.0)
                (if (<= (.MeshID (Utilities|Struct|BreakFSplineMeshEntry (Utilities|Array|Get(acopy) __roadsegments_2 (Utilities|Array|LastIndex __roadsegments_2)))) (Utilities|Array|LastIndex (LocalVariables|Get_Meshes))) ; Last segment was not replaced
                  ;;[1 1 1] Replace final segment Id with our LastMeshId
                  (bind _output_get_2 (LocalVariables|Set_CurrentMesh (Utilities|Array|Get(acopy) (LocalVariables|Get_Meshes) (Utilities|Array|LastIndex (LocalVariables|Get_Meshes)))))
                  (Utilities|Array|Add (LocalVariables|Get_RoadSegments) (Utilities|Struct|MakeFSplineMeshEntry 0 (LocalVariables|Get_LastMeshT) _output_get_2 _returnvalue_3 (LocalVariables|Get_T)))
                  (LocalVariables|Set_T (+ (LocalVariables|Get_T) (LocalVariables|Get_LastMeshT)))))
              (else
                ;[1 1 1] SetMeshT
                (Utilities|Array|Add (LocalVariables|Get_RoadSegments) (Utilities|Struct|MakeFSplineMeshEntry 0 (CallFunction|GetMeshT (LocalVariables|Get_CurrentMesh)) (LocalVariables|Get_CurrentMesh) _returnvalue_3 (LocalVariables|Get_T)))
                ;[1 1 1] Increase T
                (LocalVariables|Set_T (+ (LocalVariables|Get_T) (CallFunction|GetMeshT (LocalVariables|Get_CurrentMesh)))))))
          (:then_3
            ;[1 1 1] Safe abort while loop
            (bind _result (Math|Integer|IncrementInt (LocalVariables|Get_Counter))
              (:%20%20
                (if (> _result 1000)
                  (LocalVariables|SetbLoop false)))))))
      (return (LocalVariables|Get_RoadSegments) (/ (/ (Utilities|GetSplineLength) (Spline|GetSplineLength (Utilities|GetSpline))) (LocalVariables|Get_T))))))

(fn SpawnSplineMeshes
  (params (RoadSegments :type Array%20of%20F%20Spline%20Mesh%20Entry%20Structures) (Offset :type Vector%202D%20Structure) (StartOffset :type Float%20%28double-precision%29) (EndOffset :type Float%20%28double-precision%29) (Anchor :type EAnchor%20Enum :default "NewEnumerator3") (AnchorRight :type Boolean) (Mirror :type Boolean) (Reverse :type Boolean) (ScaleMesh :type Boolean) (ScaleOffset :type Boolean) (Smooth :type Boolean) (Rescale :type Float%20%28double-precision%29))
  (bind _returnvalue (Components|GetOwner))
  (bind _spline (Utilities|GetSpline))
  (bind _spline_2 (Utilities|GetSpline))
  (bind _spline_3 (Utilities|GetSpline))
  (bind _components (Variables|Core|GetComponents))
  (bind _components_2 (Variables|Core|GetComponents))
  (bind _bsmoothinterp (Variables|SplineMesh|GetbSmoothInterp))
  (bind _returnvalue_2 (Utilities|Array|LastIndex _components_2))
  (bind _returnvalue_3 (Class|KismetMathLibrary|XORBoolean Mirror Reverse))
  (bind _returnvalue_4 (Spline|GetSplineLength _spline_2))
  (bind _returnvalue_5 (select _bsmoothinterp "/Game/SnappyRoads/Blueprints/Core/Components/BP_SplineMesh_SmoothInterp_Component.BP_SplineMesh_SmoothInterp_Component_C" "/Script/Engine.SplineMeshComponent"))
  (LocalVariables|SetStartOffset_ (Math|Float|SelectFloat EndOffset StartOffset Reverse))
  (for _index (range 0 (Utilities|Array|LastIndex RoadSegments)) ; ForEachSegment
    (bind _output_get (LocalVariables|Set_Index _index))
    (Utilities|FlowControl|Sequence
      (:then_0
        ;[1 1 1] Add or Reuse Spline Mesh Components
        (if (Utilities|Array|IsValidIndex _components (Math|Integer|SelectInt (+ (Utilities|Array|Length RoadSegments) (LocalVariables|Get_Index)) (LocalVariables|Get_Index) Mirror))
          (Utilities|IsValid (Utilities|Array|Get(acopy) _components (Math|Integer|SelectInt (+ (Utilities|Array|Length RoadSegments) (LocalVariables|Get_Index)) (LocalVariables|Get_Index) Mirror))
            (:Is%20Valid
              (bind _output_get_2 (LocalVariables|SetSplineMeshComp_ (Utilities|Array|Get(acopy) _components (Math|Integer|SelectInt (+ (Utilities|Array|Length RoadSegments) (LocalVariables|Get_Index)) (LocalVariables|Get_Index) Mirror))))
              (Rendering|SetVisibility _output_get_2 true false)
              ;;[1 1 1] Reset Scale
              (SplineMesh|SetEndScale (LocalVariables|GetSplineMeshComp_) "(X=1.000000,Y=1.000000)" false :!class /Script/Engine.SplineMeshComponent)
              (SplineMesh|SetStartScale (LocalVariables|GetSplineMeshComp_) "(X=1.000000,Y=1.000000)" false :!class /Script/Engine.SplineMeshComponent))
            (:Is%20Not%20Valid
              (bind _returnvalue_6 (Game|AddComponentbyClass _returnvalue _returnvalue_5)) ; Faster than from AddComponent category
              (LocalVariables|SetSplineMeshComp_ (.As样条网格体组件 (Utilities|Casting|CastToSplineMeshComponent _returnvalue_6)))
              (Utilities|Array|SetArrayElem _components (Math|Integer|SelectInt (+ (Utilities|Array|Length RoadSegments) (LocalVariables|Get_Index)) (LocalVariables|Get_Index) Mirror) (.As样条网格体组件 (Utilities|Casting|CastToSplineMeshComponent _returnvalue_6)))))
          (else
            (bind _returnvalue_7 (Game|AddComponentbyClass _returnvalue _returnvalue_5)) ; Faster than from AddComponent category
            (bind _output_get_3 (LocalVariables|SetSplineMeshComp_ (.As样条网格体组件 (Utilities|Casting|CastToSplineMeshComponent _returnvalue_7))))
            (Utilities|Array|SetArrayElem _components (Math|Integer|SelectInt (+ (Utilities|Array|Length RoadSegments) (LocalVariables|Get_Index)) (LocalVariables|Get_Index) Mirror) _output_get_3 true))))
      (:then_1
        (Utilities|FlowControl|Sequence
          (:then_0
            ;[1 1 1] Set Spline Mesh Points
            ;;[1 1 1] Segment Start
            (bind _output_get_4 (LocalVariables|SetSegStart (Math|Float|SelectFloat (- _returnvalue_4 (+ (LocalVariables|GetStartOffset_) (* (* (.T (Utilities|Struct|BreakFSplineMeshEntry (Utilities|Array|Get(acopy) RoadSegments (LocalVariables|Get_Index)))) Rescale) _returnvalue_4))) (+ (LocalVariables|GetStartOffset_) (* (* (.T (Utilities|Struct|BreakFSplineMeshEntry (Utilities|Array|Get(acopy) RoadSegments (LocalVariables|Get_Index)))) Rescale) _returnvalue_4)) Reverse)))
            ;;[1 1 1] Segment End
            (bind _output_get_5 (LocalVariables|SetSegEnd (Math|Float|SelectFloat (- _returnvalue_4 (+ (+ (LocalVariables|GetStartOffset_) (* (* (.T (Utilities|Struct|BreakFSplineMeshEntry (Utilities|Array|Get(acopy) RoadSegments (LocalVariables|Get_Index)))) Rescale) _returnvalue_4)) (* _returnvalue_4 (* Rescale (.MeshT (Utilities|Struct|BreakFSplineMeshEntry (Utilities|Array|Get(acopy) RoadSegments (LocalVariables|Get_Index)))))))) (+ (+ (LocalVariables|GetStartOffset_) (* (* (.T (Utilities|Struct|BreakFSplineMeshEntry (Utilities|Array|Get(acopy) RoadSegments (LocalVariables|Get_Index)))) Rescale) _returnvalue_4)) (* _returnvalue_4 (* Rescale (.MeshT (Utilities|Struct|BreakFSplineMeshEntry (Utilities|Array|Get(acopy) RoadSegments (LocalVariables|Get_Index))))))) Reverse)))
            ;;[1 1 1] SegLength
            (bind _output_get_6 (LocalVariables|Set_SegLen (- _output_get_5 _output_get_4)))
            (SplineMesh|SetStartandEnd (LocalVariables|GetSplineMeshComp_) (.Location (Math|Transform|BreakTransform (Spline|GetTransformatDistanceAlongSpline (Utilities|GetSpline) _output_get_4 "Local" false))) (* (Math|Vector|GetForwardVector (.Rotation (Math|Transform|BreakTransform (Spline|GetTransformatDistanceAlongSpline (Utilities|GetSpline) _output_get_4 "Local" false)))) _output_get_6) (.Location (Math|Transform|BreakTransform (Spline|GetTransformatDistanceAlongSpline (Utilities|GetSpline) _output_get_5 "Local" false))) (* (Math|Vector|GetForwardVector (.Rotation (Math|Transform|BreakTransform (Spline|GetTransformatDistanceAlongSpline (Utilities|GetSpline) _output_get_5 "Local" false)))) _output_get_6) false :!class /Script/Engine.SplineMeshComponent))
          (:then_1
            (if (Variables|Spline|GetbTwistFix)
              ;[1 1 1] Twist Fix Roll
              (Class|SplineMeshComponent|SetStartRoll (LocalVariables|GetSplineMeshComp_) (Math|Float|SelectFloat (- 0.0 (Math|Trig|DegreesToRadians (.roll (Math|Rotator|CombineRotators (Spline|GetRotationatDistanceAlongSpline _spline_3 (LocalVariables|GetSegStart) "Local") (Class|KismetMathLibrary|NegateRotator (Spline|GetRotationatDistanceAlongSpline _spline_3 (+ (LocalVariables|GetSegStart) (* (LocalVariables|Get_SegLen) 0.5)) "Local")))))) (Math|Trig|DegreesToRadians (.roll (Math|Rotator|CombineRotators (Spline|GetRotationatDistanceAlongSpline _spline_3 (LocalVariables|GetSegStart) "Local") (Class|KismetMathLibrary|NegateRotator (Spline|GetRotationatDistanceAlongSpline _spline_3 (+ (LocalVariables|GetSegStart) (* (LocalVariables|Get_SegLen) 0.5)) "Local"))))) Reverse) false)
              (SplineMesh|SetSplineUpDir (LocalVariables|GetSplineMeshComp_) (.Z (Math|Rotator|GetAxes (Spline|GetRotationatDistanceAlongSpline _spline_3 (+ (LocalVariables|GetSegStart) (* (LocalVariables|Get_SegLen) 0.5)) "Local"))) false)
              (Class|SplineMeshComponent|SetEndRoll (LocalVariables|GetSplineMeshComp_) (Math|Float|SelectFloat (- 0.0 (Math|Trig|DegreesToRadians (.roll (Math|Rotator|CombineRotators (Spline|GetRotationatDistanceAlongSpline _spline_3 (LocalVariables|GetSegEnd) "Local") (Class|KismetMathLibrary|NegateRotator (Spline|GetRotationatDistanceAlongSpline _spline_3 (+ (LocalVariables|GetSegStart) (* (LocalVariables|Get_SegLen) 0.5)) "Local")))))) (Math|Trig|DegreesToRadians (.roll (Math|Rotator|CombineRotators (Spline|GetRotationatDistanceAlongSpline _spline_3 (LocalVariables|GetSegEnd) "Local") (Class|KismetMathLibrary|NegateRotator (Spline|GetRotationatDistanceAlongSpline _spline_3 (+ (LocalVariables|GetSegStart) (* (LocalVariables|Get_SegLen) 0.5)) "Local"))))) Reverse) false)
              (else
                ;[1 1 1] Simple Roll
                (Class|SplineMeshComponent|SetStartRoll (LocalVariables|GetSplineMeshComp_) (Math|Float|SelectFloat (- 0.0 (Math|Trig|DegreesToRadians (.roll (Spline|GetRotationatDistanceAlongSpline _spline (LocalVariables|GetSegStart) "Local")))) (Math|Trig|DegreesToRadians (.roll (Spline|GetRotationatDistanceAlongSpline _spline (LocalVariables|GetSegStart) "Local"))) Reverse) false)
                (Class|SplineMeshComponent|SetEndRoll (LocalVariables|GetSplineMeshComp_) (Math|Float|SelectFloat (- 0.0 (Math|Trig|DegreesToRadians (.roll (Spline|GetRotationatDistanceAlongSpline _spline (LocalVariables|GetSegEnd) "Local")))) (Math|Trig|DegreesToRadians (.roll (Spline|GetRotationatDistanceAlongSpline _spline (LocalVariables|GetSegEnd) "Local"))) Reverse) false))))
          (:then_2
            (if ScaleMesh ; UseScale, scale mesh and offsets
              ;[1 1 1] Scale
              (SplineMesh|SetStartScale (LocalVariables|GetSplineMeshComp_) (Math|Vector2D|MakeVector2D (.x (Utilities|GetScaleatDistance (LocalVariables|GetSegStart))) (.y (Utilities|GetScaleatDistance (LocalVariables|GetSegStart)))) false :!class /Script/Engine.SplineMeshComponent)
              (SplineMesh|SetEndScale (LocalVariables|GetSplineMeshComp_) (Math|Vector2D|MakeVector2D (.x (Utilities|GetScaleatDistance (LocalVariables|GetSegEnd))) (.y (Utilities|GetScaleatDistance (LocalVariables|GetSegEnd)))) false :!class /Script/Engine.SplineMeshComponent)))
          (:then_3
            ;[1 1 1] Offset & Roll Pivot Shift/Fix
            (SplineMesh|SetStartOffset (LocalVariables|GetSplineMeshComp_) (Class|KismetMathLibrary|GetRotated2D (Math|Vector2D|MakeVector2D (.ScaledOffsetX (Utilities|GetOffsetatDistance (LocalVariables|GetSegStart) _returnvalue_3)) (.ScaledOffsetY (Utilities|GetOffsetatDistance (LocalVariables|GetSegStart) _returnvalue_3))) (- 0.0 (Math|Trig|RadiansToDegrees (SplineMesh|GetStartRoll (LocalVariables|GetSplineMeshComp_))))) false)
            (SplineMesh|SetEndOffset (LocalVariables|GetSplineMeshComp_) (Class|KismetMathLibrary|GetRotated2D (Math|Vector2D|MakeVector2D (.ScaledOffsetX (Utilities|GetOffsetatDistance (LocalVariables|GetSegEnd) _returnvalue_3)) (.ScaledOffsetY (Utilities|GetOffsetatDistance (LocalVariables|GetSegEnd) _returnvalue_3))) (- 0.0 (Math|Trig|RadiansToDegrees (SplineMesh|GetEndRoll (LocalVariables|GetSplineMeshComp_))))) false))
          (:then_4
            ;[1 1 1] Deprecated
            (if Reverse
              _))
          (:then_6
            ;[1 1 1] Cosmetics
            ;;[1 1 1] ApplySegmentScale
            (SplineMesh|SetStartScale (LocalVariables|GetSplineMeshComp_) (* (SplineMesh|GetStartScale (LocalVariables|GetSplineMeshComp_)) (.Scale (Utilities|Struct|BreakFSplineMeshEntry (Utilities|Array|Get(acopy) RoadSegments (Math|Integer|%(Integer) _output_get (Utilities|Array|Length RoadSegments)))))) false :!class /Script/Engine.SplineMeshComponent)
            (SplineMesh|SetEndScale (LocalVariables|GetSplineMeshComp_) (* (SplineMesh|GetEndScale (LocalVariables|GetSplineMeshComp_)) (.Scale (Utilities|Struct|BreakFSplineMeshEntry (Utilities|Array|Get(acopy) RoadSegments (Math|Integer|%(Integer) _output_get (Utilities|Array|Length RoadSegments)))))) false :!class /Script/Engine.SplineMeshComponent)
            (SplineMesh|SetForwardAxis (LocalVariables|GetSplineMeshComp_) (Variables|Mesh|GetForwardAxis) false)
            (Utilities|SetMaterialOverrides (LocalVariables|GetSplineMeshComp_) (LocalVariables|GetSegStart) (LocalVariables|Get_SegLen))
            (Utilities|SetMeshProperties (LocalVariables|GetSplineMeshComp_) (.SplineMesh (Utilities|Struct|BreakFSplineMeshEntry (Utilities|Array|Get(acopy) RoadSegments (Math|Integer|%(Integer) _output_get (Utilities|Array|Length RoadSegments)))))))))))
  (if (< (Math|Integer|SelectInt (+ (Utilities|Array|Length RoadSegments) (LocalVariables|Get_Index)) (LocalVariables|Get_Index) Mirror) _returnvalue_2) ; Still have extra components left?
    ;[1 1 1] Hide unused extra comps, will be destroyed on the next run of the construction script
    (for _index_2 (range (+ (Math|Integer|SelectInt (+ (Utilities|Array|Length RoadSegments) (LocalVariables|Get_Index)) (LocalVariables|Get_Index) Mirror) 1) _returnvalue_2)
      (Rendering|SetVisibility (Utilities|Array|Get(acopy) _components_2 _index_2) false false)))
  ;[1 1 1] Finish
  (return))

(fn SwapFirstandLast
  (params (MeshSegments :type Array%20of%20F%20Spline%20Mesh%20Entry%20Structures))
  (bind _splinemeshsettings (Variables|SplineMesh|GetSplineMeshSettings))
  (bind _meshes (Utilities|Struct|BreakFSplineMeshStettings _splinemeshsettings))
  (Utilities|Struct|SetmembersinFSplineMeshEntry (Utilities|Array|Get(acopy) MeshSegments) (Utilities|Array|Get(acopy) _meshes 2))
  (Utilities|Struct|SetmembersinFSplineMeshEntry (Utilities|Array|Get(acopy) MeshSegments (Utilities|Array|LastIndex MeshSegments)) (Utilities|Array|Get(acopy) _meshes 1))
  (return MeshSegments))