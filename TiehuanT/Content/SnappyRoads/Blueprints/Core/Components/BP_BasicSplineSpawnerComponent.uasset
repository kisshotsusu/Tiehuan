(event EventRun
  (CallFunction|Build))

(fn Build
  (bind _meshextrasettings (Variables|Default|GetMeshExtraSettings))
  (bind _points (CallFunction|SplineSampler (Utilities|GetSpline) (Variables|Default|GetMeshExtraSettings)))
  (CallFunction|AddMeshes _meshextrasettings _points)
  ;[1 1 1] Mirror
  (if (.Mirror (Utilities|Struct|BreakFMeshExtraSettings _meshextrasettings)) ; Mirror?
    (bind _structout (Utilities|Struct|SetmembersinFMeshExtraSettings _meshextrasettings false))
    (bind _points_2 (CallFunction|SplineSampler (Utilities|GetSpline) _structout))
    (CallFunction|AddMeshes _structout _points_2)))

(fn AddMeshes
  (params (MeshExtraOptions :type F%20Mesh%20Extra%20Settings%20Structure) (Points :type Array%20of%20Transforms))
  (bind (_spawner _mesh _actor _spacing _offset _rotationz _snaptofloor _snaptoedge _mirror _invert _keepvertical _usesplinescale _positionvariation _rotationvariation _maxdrawdistance) (Utilities|Struct|BreakFMeshExtraSettings MeshExtraOptions))
  (Utilities|FlowControl|Sequence
    (:then_0
      ;[1 1 1] Snap to Floor
      (if _snaptofloor
        (for (_ _array_index) Points
          (CallFunction|StretchtoFloor (Utilities|Array|Get(acopy) Points _array_index)))))
    (:then_1
      (if (Utilities|IsValid _mesh)
        (bind _returnvalue (Game|AddComponentbyClass (Components|GetOwner) "/Script/Engine.HierarchicalInstancedStaticMeshComponent" false))
        ;[1 1 1] Configure component
        (Components|StaticMesh|SetStaticMesh _returnvalue _mesh)
        (Class|PrimitiveComponent|SetCullDistance _returnvalue _maxdrawdistance)
        (Transformation|SetMobility _returnvalue "Static")
        (Components|InstancedStaticMesh|AddInstances _returnvalue Points false false)))
    (:then_2
      ;[1 1 1] Add child actors
      (if (Utilities|IsValidClass _actor)
        (for _array_element Points
          (bind _returnvalue_2 (Game|AddComponentbyClass (Components|GetOwner) "/Script/Engine.ChildActorComponent" false _array_element))
          (ChildActorComponent|SetChildActorClass _returnvalue_2 _actor))))))

(fn SplineSampler
  (params (Spline :type Spline%20Component%20Object%20Reference) (FMeshExtraSettings :type F%20Mesh%20Extra%20Settings%20Structure%20%28by%20ref%29))
  (bind (_spawner _mesh _actor _spacing _offset _rotationz _snaptofloor _snaptoedge _mirror _invert _keepvertical _usesplinescale _positionvariation _rotationvariation) (Utilities|Struct|BreakFMeshExtraSettings FMeshExtraSettings))
  (bind _spline (Utilities|GetSpline))
  (bind _roadhalfwidth (Variables|Default|GetRoadHalfWidth))
  (bind (_x _y _z) (Math|Vector|BreakVector _positionvariation))
  (bind (_roll _pitch _yaw) (Math|Rotator|BreakRotator _rotationvariation))
  (bind _returnvalue (Utilities|RandomFloatfromStream _roll))
  (bind _returnvalue_2 (Utilities|RandomFloatfromStream _z))
  (bind _returnvalue_3 (Utilities|RandomFloatfromStream _y))
  (bind _returnvalue_4 (+ _offset (Math|Vector|MakeVector 0.0 _returnvalue_3 _returnvalue_2)))
  (bind _returnvalue_5 (* _returnvalue_4 "1.000000,-1.000000,1.000000"))
  (bind _returnvalue_6 (Math|Vector|SelectVector _returnvalue_5 _returnvalue_4 _mirror))
  (for _index (range 0 (.ReturnValue (Math|Float|Division(WholeandRemainder) (Spline|GetSplineLength Spline) _spacing)))
    (Utilities|Array|Add (LocalVariables|Get_Points) (Math|Transform|MakeTransform (Math|Transform|TransformLocation (select (Variables|Default|GetbUseRoll) (Spline|GetTransformatDistanceAlongSpline _spline (+ (Math|Float|%(Float) (+ (* _index _spacing) (.X (Math|Vector|BreakVector _offset))) (Spline|GetSplineLength _spline)) (Utilities|RandomFloatfromStream _x)) "Local" false) (Math|Transform|MakeTransform (.Location (Math|Transform|BreakTransform (Spline|GetTransformatDistanceAlongSpline _spline (+ (Math|Float|%(Float) (+ (* _index _spacing) (.X (Math|Vector|BreakVector _offset))) (Spline|GetSplineLength _spline)) (Utilities|RandomFloatfromStream _x)) "Local" false))) (Math|Rotator|MakeRotator 0.0 (.pitch (.Rotation (Math|Transform|BreakTransform (Spline|GetTransformatDistanceAlongSpline _spline (+ (Math|Float|%(Float) (+ (* _index _spacing) (.X (Math|Vector|BreakVector _offset))) (Spline|GetSplineLength _spline)) (Utilities|RandomFloatfromStream _x)) "Local" false)))) (.yaw (.Rotation (Math|Transform|BreakTransform (Spline|GetTransformatDistanceAlongSpline _spline (+ (Math|Float|%(Float) (+ (* _index _spacing) (.X (Math|Vector|BreakVector _offset))) (Spline|GetSplineLength _spline)) (Utilities|RandomFloatfromStream _x)) "Local" false))))) (.Scale (Math|Transform|BreakTransform (Spline|GetTransformatDistanceAlongSpline _spline (+ (Math|Float|%(Float) (+ (* _index _spacing) (.X (Math|Vector|BreakVector _offset))) (Spline|GetSplineLength _spline)) (Utilities|RandomFloatfromStream _x)) "Local" false))))) (+ (* (Math|Vector|SelectVector (Math|Vector|MakeVector 0.0 (Math|Float|SelectFloat (- 0.0 _roadhalfwidth) _roadhalfwidth _mirror) 0.0) _returnvalue_6 _snaptoedge) (Math|Vector|MakeVector 0.0 (.x (Utilities|GetRoadScale (+ (Math|Float|%(Float) (+ (* _index _spacing) (.X (Math|Vector|BreakVector _offset))) (Spline|GetSplineLength _spline)) (Utilities|RandomFloatfromStream _x)))) (.y (Utilities|GetRoadScale (+ (Math|Float|%(Float) (+ (* _index _spacing) (.X (Math|Vector|BreakVector _offset))) (Spline|GetSplineLength _spline)) (Utilities|RandomFloatfromStream _x)))))) (Math|Vector|SelectVector _returnvalue_6 "0, 0, 0" _snaptoedge))) (Math|Rotator|SelectRotator (Math|Rotator|MakeRotator _returnvalue 0.0 (.Yaw (Math|Rotator|BreakRotator (Math|Transform|TransformRotation (select (Variables|Default|GetbUseRoll) (Spline|GetTransformatDistanceAlongSpline _spline (+ (Math|Float|%(Float) (+ (* _index _spacing) (.X (Math|Vector|BreakVector _offset))) (Spline|GetSplineLength _spline)) (Utilities|RandomFloatfromStream _x)) "Local" false) (Math|Transform|MakeTransform (.Location (Math|Transform|BreakTransform (Spline|GetTransformatDistanceAlongSpline _spline (+ (Math|Float|%(Float) (+ (* _index _spacing) (.X (Math|Vector|BreakVector _offset))) (Spline|GetSplineLength _spline)) (Utilities|RandomFloatfromStream _x)) "Local" false))) (Math|Rotator|MakeRotator 0.0 (.pitch (.Rotation (Math|Transform|BreakTransform (Spline|GetTransformatDistanceAlongSpline _spline (+ (Math|Float|%(Float) (+ (* _index _spacing) (.X (Math|Vector|BreakVector _offset))) (Spline|GetSplineLength _spline)) (Utilities|RandomFloatfromStream _x)) "Local" false)))) (.yaw (.Rotation (Math|Transform|BreakTransform (Spline|GetTransformatDistanceAlongSpline _spline (+ (Math|Float|%(Float) (+ (* _index _spacing) (.X (Math|Vector|BreakVector _offset))) (Spline|GetSplineLength _spline)) (Utilities|RandomFloatfromStream _x)) "Local" false))))) (.Scale (Math|Transform|BreakTransform (Spline|GetTransformatDistanceAlongSpline _spline (+ (Math|Float|%(Float) (+ (* _index _spacing) (.X (Math|Vector|BreakVector _offset))) (Spline|GetSplineLength _spline)) (Utilities|RandomFloatfromStream _x)) "Local" false))))) (Math|Rotator|MakeRotator _returnvalue 0.0 (+ (Math|Float|SelectFloat (+ _rotationz 1.8e+02) _rotationz _mirror) (Utilities|RandomFloatfromStream _yaw))))))) (Math|Transform|TransformRotation (select (Variables|Default|GetbUseRoll) (Spline|GetTransformatDistanceAlongSpline _spline (+ (Math|Float|%(Float) (+ (* _index _spacing) (.X (Math|Vector|BreakVector _offset))) (Spline|GetSplineLength _spline)) (Utilities|RandomFloatfromStream _x)) "Local" false) (Math|Transform|MakeTransform (.Location (Math|Transform|BreakTransform (Spline|GetTransformatDistanceAlongSpline _spline (+ (Math|Float|%(Float) (+ (* _index _spacing) (.X (Math|Vector|BreakVector _offset))) (Spline|GetSplineLength _spline)) (Utilities|RandomFloatfromStream _x)) "Local" false))) (Math|Rotator|MakeRotator 0.0 (.pitch (.Rotation (Math|Transform|BreakTransform (Spline|GetTransformatDistanceAlongSpline _spline (+ (Math|Float|%(Float) (+ (* _index _spacing) (.X (Math|Vector|BreakVector _offset))) (Spline|GetSplineLength _spline)) (Utilities|RandomFloatfromStream _x)) "Local" false)))) (.yaw (.Rotation (Math|Transform|BreakTransform (Spline|GetTransformatDistanceAlongSpline _spline (+ (Math|Float|%(Float) (+ (* _index _spacing) (.X (Math|Vector|BreakVector _offset))) (Spline|GetSplineLength _spline)) (Utilities|RandomFloatfromStream _x)) "Local" false))))) (.Scale (Math|Transform|BreakTransform (Spline|GetTransformatDistanceAlongSpline _spline (+ (Math|Float|%(Float) (+ (* _index _spacing) (.X (Math|Vector|BreakVector _offset))) (Spline|GetSplineLength _spline)) (Utilities|RandomFloatfromStream _x)) "Local" false))))) (Math|Rotator|MakeRotator _returnvalue 0.0 (+ (Math|Float|SelectFloat (+ _rotationz 1.8e+02) _rotationz _mirror) (Utilities|RandomFloatfromStream _yaw)))) _keepvertical) (Math|Vector|SelectVector (Math|Vector|MakeVector 1.0 (.x (Utilities|GetRoadScale (+ (Math|Float|%(Float) (+ (* _index _spacing) (.X (Math|Vector|BreakVector _offset))) (Spline|GetSplineLength _spline)) (Utilities|RandomFloatfromStream _x)))) 1.0) "1.000000,1.000000,1.000000" _usesplinescale))))
  (return (LocalVariables|Get_Points)))

(fn StretchtoFloor
  (params (Transform :type Transform%20%28by%20ref%29))
  (bind _returnvalue (Components|GetOwner))
  (bind _location (Math|Transform|BreakTransform Transform))
  (bind _meshextrasettings (Variables|Default|GetMeshExtraSettings))
  (bind _mesh (Utilities|Struct|BreakFMeshExtraSettings _meshextrasettings))
  (bind _returnvalue_2 (Transformation|GetActorTransform _returnvalue))
  (bind _returnvalue_3 (StaticMesh|GetBoundingBox _mesh))
  (bind _returnvalue_4 (+ (.location _returnvalue_2) _location))
  (bind _z (Math|Vector|BreakVector (.min _returnvalue_3)))
  (bind _outhits (Class|KismetSystemLibrary|LineTraceMultiforObjects _returnvalue_4 (+ _returnvalue_4 (Math|Vector|MakeVector 0.0 0.0 (* _z 3.0)) "") (Utilities|Array|MakeArray "ObjectTypeQuery1") false 0 "ForOneFrame" true))
  (for _array_element _outhits
    (Utilities|Casting|CastToLandscape (.HitActor (Collision|BreakHitResult _array_element)))
    (|SetBy-RefVar Transform (Math|Transform|ComposeTransforms (Math|Transform|MakeTransform "0, 0, 0" "0, 0, 0" (Math|Vector|MakeVector 1.0 1.0 (Math|Float|Absolute(Float) (/ (.Distance (Collision|BreakHitResult _array_element)) _z)))) Transform))))