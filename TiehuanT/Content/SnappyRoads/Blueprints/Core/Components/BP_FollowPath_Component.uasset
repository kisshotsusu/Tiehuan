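; Component that drives its owning vehicle along a spline in a continuous loop, optionally in reverse.
; On BeginPlay it makes a few random attempts at a start distance clear of other BP_SimpleVehicle actors, or disables ticking without a valid spline.
; Each tick it teleports the owner along the spline and steps speed toward the target, braking while CollidingVehicle is valid.
; A forward line trace is unfinished and disabled.
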(event EventBeginPlay
  (bind _spline (Variables|Core|GetSpline))
  (bind _spline_2 (Variables|Core|GetSpline))
  ;[1 1 1] ValidityCheck
  (Utilities|IsValid _spline_2
    (:Is%20Valid
      (bind _output_get (Variables|Core|SetLength (Spline|GetSplineLength _spline_2)))
      (if (> _output_get 0.0)
        ;[1 1 1] [Move2VehiclesOBP] PlaceRandomlyAlongTheSplineAvoidingOverlaps
        (bind _index (Utilities|FlowControl|ForLoopwithBreak 0 5 :!label _label)
          (:LoopBody
            (bind _output_get_2 (Variables|Core|Set_temp (Math|Random|RandomFloatinRange 0.0 (- _output_get 6e+02))))
            (bind _returnvalue (Collision|SphereOverlapActors (+ (Spline|GetLocationatDistanceAlongSpline _spline _output_get_2 "World") (Math|Vector|RotateVector (Variables|Config|GetOffset) (Spline|GetRotationatDistanceAlongSpline _spline _output_get_2 "World"))) 3e+02 (Utilities|Array|MakeArray "ObjectTypeQuery2") "/Game/SnappyRoads/Blueprints/Vehicle/BP_SimpleVehicle.BP_SimpleVehicle_C"))
            (if (not _returnvalue)
              (goto _label Break)))
          (:Completed
            (Variables|Core|SetCurrentDistance _output_get_2)
            ;[1 1 1] Movement
            (Transformation|SetActorLocationAndRotation (Components|GetOwner) (.location (Spline|GetTransformatDistanceAlongSpline (Variables|Core|GetSpline) (Math|Float|SelectFloat (- (Variables|Core|GetLength) (Variables|Core|GetCurrentDistance)) (Variables|Core|GetCurrentDistance) (Variables|Default|GetReverse)) "World" false)) (.rotation (Spline|GetTransformatDistanceAlongSpline (Variables|Core|GetSpline) (Math|Float|SelectFloat (- (Variables|Core|GetLength) (Variables|Core|GetCurrentDistance)) (Variables|Core|GetCurrentDistance) (Variables|Default|GetReverse)) "World" false)) false true)
            (Variables|Core|SetCurrentDistance (Math|Float|%(Float) (+ (* (stale EventTick DeltaSeconds) (Variables|Config|GetCurrentSpeed) 25.0) (Variables|Core|GetCurrentDistance)) (Variables|Core|GetLength)))))
        (else
          (Components|Tick|SetComponentTickEnabled false :!label _label_2))))
    (:Is%20Not%20Valid
      (goto _label_2))))

(event EventTick
  (params (DeltaSeconds :type Float%20%28single-precision%29))
  (bind _returnvalue (Components|GetOwner))
  (bind _speed (Variables|Config|GetSpeed))
  (bind _asbp_simple_vehicle (Utilities|Casting|CastToBP_SimpleVehicle _returnvalue))
  (bind _offset (Variables|/Game/SnappyRoads/Blueprints/Vehicle/BP_SimpleVehicle.BP_SimpleVehicle_C|GetOffset _asbp_simple_vehicle))
  (bind _returnvalue_2 (Transformation|GetWorldLocation _offset))
  (bind _returnvalue_3 (+ _returnvalue_2 "0, 0,50.000000"))
  (Utilities|FlowControl|Sequence
    (:then_0
      ;[1 1 1] LineTrace_WIP
      (if false
        (Collision|LineTraceForObjects _returnvalue_3 (+ _returnvalue_3 (* (Math|Vector|GetForwardVector (Transformation|GetWorldRotation _offset)) 1e+03)) (Utilities|Array|MakeArray "ObjectTypeQuery5") false 0 "ForOneFrame")))
    (:then_1
      ;[1 1 1] Movement
      (Transformation|SetActorLocationAndRotation (Components|GetOwner) (.location (Spline|GetTransformatDistanceAlongSpline (Variables|Core|GetSpline) (Math|Float|SelectFloat (- (Variables|Core|GetLength) (Variables|Core|GetCurrentDistance)) (Variables|Core|GetCurrentDistance) (Variables|Default|GetReverse)) "World" false)) (.rotation (Spline|GetTransformatDistanceAlongSpline (Variables|Core|GetSpline) (Math|Float|SelectFloat (- (Variables|Core|GetLength) (Variables|Core|GetCurrentDistance)) (Variables|Core|GetCurrentDistance) (Variables|Default|GetReverse)) "World" false)) false true)
      (Variables|Core|SetCurrentDistance (Math|Float|%(Float) (+ (* DeltaSeconds (Variables|Config|GetCurrentSpeed) 25.0) (Variables|Core|GetCurrentDistance)) (Variables|Core|GetLength))))
    (:then_2
      ;[1 1 1] ManageSpeed
      (if (or (> (Variables|Config|GetCurrentSpeed) _speed) (Utilities|IsValid (Variables|/Game/SnappyRoads/Blueprints/Vehicle/BP_SimpleVehicle.BP_SimpleVehicle_C|GetCollidingVehicle _asbp_simple_vehicle)))
        (Variables|Config|SetCurrentSpeed (Math|Float|Clamp(Float) (+ (Variables|Config|GetCurrentSpeed) -0.25) 0.0 1e+03))
        (elif (< (Variables|Config|GetCurrentSpeed) _speed)
          (Variables|Config|SetCurrentSpeed (+ (Variables|Config|GetCurrentSpeed) 0.25)))))))