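; Spline-based fence builder that lays out a mesh along straight segments in the construction script.
; Each segment gets a rounded count of pieces, stretched to fit between corner offsets and added to a hierarchical instanced mesh.
; KeepLevel keeps pieces upright by using yaw only and horizontal length, rescaled to spline distance.
; An optional PointMesh is instanced at every spline point or placed only at the last one.
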(event Custom|Build
  (bind _spline (Variables|Default|GetSpline))
  (bind _returnvalue (Class|SplineComponent|GetNumberOfSplineSegments _spline))
  (bind _returnvalue_2 (- _returnvalue 1))
  (bind _returnvalue_3 (Spline|GetTransformatSplinePoint _spline _returnvalue_2 "Local" true))
  (Utilities|FlowControl|Sequence
    (:then_0
      (bind _returnvalue_4 (AddComponent|AddHierarchicalInstancedStaticMeshComponent false))
      (Components|StaticMesh|SetStaticMesh _returnvalue_4 (Variables|Default|GetMesh)))
    (:then_1
      (Utilities|Array|Clear (Variables|Debug|GetTransforms))
      (for _index (range 0 (- (Class|SplineComponent|GetNumberOfSplineSegments (Variables|Default|GetSpline)) 1))
        (bind _points (CallFunction|SampleSegment _index))
        (Utilities|Array|AppendArray (Variables|Debug|GetTransforms) _points))
      (Components|InstancedStaticMesh|AddInstances _returnvalue_4 (Variables|Debug|GetTransforms) false false))
    (:then_2
      (Variables|Default|GetPointMesh
        (:then
          (if (Variables|Default|GetbMeshAtLastPointOnly)
            (bind _returnvalue_5 (AddComponent|AddStaticMeshComponent false (Math|Transform|MakeTransform (Spline|GetLocationatSplinePoint _spline _returnvalue "Local") (.rotation _returnvalue_3) (.scale _returnvalue_3))))
            (Components|StaticMesh|SetStaticMesh _returnvalue_5 (Variables|Default|GetPointMesh))
            (else
              (Utilities|FlowControl|Sequence
                (:then_0
                  (bind _returnvalue_6 (AddComponent|AddHierarchicalInstancedStaticMeshComponent false))
                  (Components|StaticMesh|SetStaticMesh _returnvalue_6 (Variables|Default|GetPointMesh)))
                (:then_1
                  (bind _points_2 (CallFunction|SampleSplinePoints))
                  (Components|InstancedStaticMesh|AddInstances _returnvalue_6 _points_2 false false))))))
        (:else)))))

(fn ConstructionScript
  (bind _spline (Variables|Default|GetSpline))
  (Utilities|FlowControl|Sequence
    (:then_0
      ;[1 1 1] SetLinear
      (for _index (range 0 (Class|SplineComponent|GetNumberOfSplineSegments _spline))
        (Spline|SetSplinePointType _spline _index "Linear" false)))
    (:then_1
      (CallFunction|Build))))

(fn SampleSegment
  (params (Segment :type Integer))
  (bind _returnvalue (Utilities|GetMeshLength))
  (bind (_length _rescale) (CallFunction|GetSegLength Segment))
  (for _index (range 0 (- (Math|Float|Round (/ (- _length (* (Variables|Default|GetCornerOffset) 2.0)) _returnvalue)) 1))
    (Utilities|Array|Add (LocalVariables|GetPoints_) (Math|Transform|ComposeTransforms (Math|Transform|MakeTransform (Math|Vector|MakeVector (* _returnvalue -0.5) 0.0 0.0) "0, 0, 0" (Math|Vector|MakeVector (/ (- _length (* (Variables|Default|GetCornerOffset) 2.0)) (* (Math|Float|Round (/ (- _length (* (Variables|Default|GetCornerOffset) 2.0)) _returnvalue)) _returnvalue)) 1.0 1.0)) (Math|Transform|MakeTransform (.Location (Math|Transform|BreakTransform (Spline|GetTransformatDistanceAlongSpline (Variables|Default|GetSpline) (+ (Spline|GetDistanceAlongSplineatSplinePoint (Variables|Default|GetSpline) Segment) (Variables|Default|GetCornerOffset) (* (* _index _returnvalue) (/ (- _length (* (Variables|Default|GetCornerOffset) 2.0)) (* (Math|Float|Round (/ (- _length (* (Variables|Default|GetCornerOffset) 2.0)) _returnvalue)) _returnvalue)) _rescale) (* _returnvalue 0.5)) "Local" true))) (Math|Rotator|SelectRotator (Math|Rotator|MakeRotator 0.0 0.0 (.Yaw (Math|Rotator|BreakRotator (.Rotation (Math|Transform|BreakTransform (Spline|GetTransformatDistanceAlongSpline (Variables|Default|GetSpline) (+ (Spline|GetDistanceAlongSplineatSplinePoint (Variables|Default|GetSpline) Segment) (Variables|Default|GetCornerOffset) (* (* _index _returnvalue) (/ (- _length (* (Variables|Default|GetCornerOffset) 2.0)) (* (Math|Float|Round (/ (- _length (* (Variables|Default|GetCornerOffset) 2.0)) _returnvalue)) _returnvalue)) _rescale) (* _returnvalue 0.5)) "Local" true)))))) (.Rotation (Math|Transform|BreakTransform (Spline|GetTransformatDistanceAlongSpline (Variables|Default|GetSpline) (+ (Spline|GetDistanceAlongSplineatSplinePoint (Variables|Default|GetSpline) Segment) (Variables|Default|GetCornerOffset) (* (* _index _returnvalue) (/ (- _length (* (Variables|Default|GetCornerOffset) 2.0)) (* (Math|Float|Round (/ (- _length (* (Variables|Default|GetCornerOffset) 2.0)) _returnvalue)) _returnvalue)) _rescale) (* _returnvalue 0.5)) "Local" true))) (Variables|Default|GetbKeepLevel)) (.Scale (Math|Transform|BreakTransform (Spline|GetTransformatDistanceAlongSpline (Variables|Default|GetSpline) (+ (Spline|GetDistanceAlongSplineatSplinePoint (Variables|Default|GetSpline) Segment) (Variables|Default|GetCornerOffset) (* (* _index _returnvalue) (/ (- _length (* (Variables|Default|GetCornerOffset) 2.0)) (* (Math|Float|Round (/ (- _length (* (Variables|Default|GetCornerOffset) 2.0)) _returnvalue)) _returnvalue)) _rescale) (* _returnvalue 0.5)) "Local" true)))))))
  (return (LocalVariables|GetPoints_)))

(fn SampleSplinePoints
  (bind _spline (Variables|Default|GetSpline))
  (for _index (range 0 (Class|SplineComponent|GetNumberOfSplineSegments _spline))
    (Utilities|Array|Add (LocalVariables|GetPoints_) (Math|Transform|ComposeTransforms (Math|Transform|MakeTransform "0, 0, 0" (Math|Rotator|MakeRotator 0.0 0.0 (Variables|Default|GetEndMeshRotationZ)) "1.000000,1.000000,1.000000") (Spline|GetTransformatDistanceAlongSpline _spline (- (Spline|GetDistanceAlongSplineatSplinePoint _spline _index) 0.1) "Local" true))))
  (return (LocalVariables|GetPoints_)))

(fn GetSegLength
  (params (Segment :type Integer))
  (bind _returnvalue (+ Segment 1))
  (bind _bkeeplevel (Variables|Default|GetbKeepLevel))
  (bind _spline (Variables|Default|GetSpline))
  (bind _returnvalue_2 (Spline|GetLocationatSplinePoint _spline Segment "Local"))
  (bind _returnvalue_3 (Spline|GetLocationatSplinePoint _spline _returnvalue "Local"))
  (bind _returnvalue_4 (Spline|GetDistanceAlongSplineatSplinePoint _spline _returnvalue))
  (bind _returnvalue_5 (Spline|GetDistanceAlongSplineatSplinePoint _spline Segment))
  (bind _returnvalue_6 (- _returnvalue_4 _returnvalue_5))
  (bind _returnvalue_7 (Math|Vector|Distance2D(Vector) _returnvalue_3 _returnvalue_2))
  (return (Math|Float|SelectFloat _returnvalue_7 _returnvalue_6 _bkeeplevel) (Math|Float|SelectFloat (/ _returnvalue_6 _returnvalue_7) 1.0 _bkeeplevel)))