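; BP_Waikuo is a construction-script tool actor that paints an outward-expanded spline band into a render target.
; It expands Spline into Spline2, meshes between them, then draws those triangles into RT and the inner spline's triangulated shape into RT2.
; Optional center fill composites RT2 with RT through a material.
; It caches location, area size and yaw as sampling parameters, with optional procedural-mesh and plane previews.
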(event EventBeginPlay
  (|CallParentFunction) ; 此节点被禁用，将不会被调用。\n从引脚连出引线来编译功能。
)

(event Collision|EventActorBeginOverlap
  (params (OtherActor :type Actor%20Object%20Reference))
  (|CallParentFunction OtherActor) ; 此节点被禁用，将不会被调用。\n从引脚连出引线来编译功能。
)

(event EventTick
  (params (DeltaSeconds :type Float%20%28single-precision%29))
  (|CallParentFunction DeltaSeconds) ; 此节点被禁用，将不会被调用。\n从引脚连出引线来编译功能。
)

(fn ConstructionScript
  (Utilities|FlowControl|Sequence
    (:then_0
      (CallFunction|样条线范围扩张 (Variables|Default|GetSpline) (Variables|Default|GetSpline2) (Variables|区域控制|Get外扩范围) (Variables|区域控制|Get切线))
      ;[1 1 1] 缓存数据
      (bind (_vertex1 _uv01 _triangles1) (CallFunction|GenMeshfromTwoSplineTwoSide (Variables|区域控制|Get采样分段) (Variables|Default|GetSpline) (Variables|Default|GetSpline2)))
      (Utilities|FlowControl|Sequence
        (:then_0
          (Variables|Cache|SetVertex%201 _vertex1))
        (:then_1
          (Variables|缓存|SetUV01 _uv01))
        (:then_2
          (Variables|缓存|SetTriangles%201 _triangles1))
        (:then_3
          (if (Variables|预览|Get预览形状)
            (Class|ProceduralMeshComponent|CreateMeshSectionLinearColor (Variables|Default|GetProceduralMesh) 0 _vertex1 _triangles1 0 _uv01 0 0 0 0 0 false false)))))
    (:then_1
      (CallFunction|绘制)
      (CallFunction|缓存传递参数))
    (:then_2
      (if (Variables|预览|Get预览颜色)
        (bind _returnvalue (Rendering|Material|CreateDynamicMaterialInstance (Variables|Default|GetPlane) 0 (Variables|预设配置|Get预览材质) "None" :!class /Script/Engine.PrimitiveComponent))
        (Rendering|Material|SetTextureParameterValue _returnvalue "RT" (Variables|参数传递|GetRT))
        (Transformation|SetRelativeScale3D (Variables|Default|GetPlane) (Math|Conversions|ToVector(Float) (Variables|区域控制|Get区域大小)))
        (else
          (Transformation|SetRelativeScale3D (Variables|Default|GetPlane) "0, 0, 0"))))))

(fn 绘制
  (params (Triangles :type Array%20of%20Canvas%20UV%20Tri%20Structures))
  (bind _rt (Variables|参数传递|GetRT))
  (bind _区域大小 (Variables|区域控制|Get区域大小))
  (bind _returnvalue (* _区域大小 1e+02))
  (bind _sizex (Variables|/Script/Engine.TextureRenderTarget2D|GetSizeX _rt))
  (bind _sizey (Variables|/Script/Engine.TextureRenderTarget2D|GetSizeY _rt))
  (bind _returnvalue_2 (Math|Integer|Max(Integer) _sizex _sizey))
  (bind _returnvalue_3 (/ _returnvalue _returnvalue_2))
  (Utilities|FlowControl|Sequence
    (:then_0
      (bind _画布1 (CallFunction|顶点转画布坐标 (Variables|Cache|GetVertex%201) (Variables|缓存|GetUV01) _returnvalue_2 _returnvalue_3 (Variables|缓存|GetTriangles%201)))
      (CallFunction|三角形渲染到渲染目标 (Variables|参数传递|GetRT) _画布1 "/Game/LibSu/Asset/Texture/T_White.T_White"))
    (:then_1
      (bind _triangles1 (CallFunction|三角形计算渲染目标 (Utilities|Array|MakeArray 0) (Utilities|Array|MakeArray (Variables|Default|GetSpline)) (* (/ (Spline|GetSplineLength (Variables|Default|GetSpline)) (Variables|区域控制|Get采样分段)) 0.01) _returnvalue_3 _returnvalue_2))
      (CallFunction|三角形渲染到渲染目标 (Variables|参数传递|GetRT2) _triangles1 "/Game/LibSu/Asset/Texture/T_White.T_White"))
    (:then_2
      (if (Variables|区域控制|Get填充中间)
        (bind _returnvalue_4 (Rendering|Material|CreateDynamicMaterialInstance "/Game/LibSu/Asset/Material/M_TextureToRendertarget.M_TextureToRendertarget" "None" "None" :!class /Script/Engine.KismetMaterialLibrary))
        (Utilities|FlowControl|Sequence
          (:then_0
            (Rendering|Material|SetTextureParameterValue _returnvalue_4 "TextureInput" (Variables|参数传递|GetRT2)))
          (:then_1
            (Rendering|Material|SetTextureParameterValue _returnvalue_4 "TextureInput2" (Variables|参数传递|GetRT)))
          (:then_2
            (Rendering|DrawMaterialtoRenderTarget (Variables|参数传递|GetRT) _returnvalue_4)))))))

(fn 缓存传递参数
  (Variables|参数传递|Set采样中心位置 (Transformation|GetActorLocation))
  (Variables|参数传递|Set采样大小 (Variables|区域控制|Get区域大小))
  (Variables|参数传递|Set采样旋转 (/ (.yaw (Transformation|GetActorRotation)) -3.6e+02)))