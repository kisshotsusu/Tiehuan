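; Editor-configurable actor that rasterizes spline areas into a render target mask, previewed on a debug mesh.
; Construction, live or manually triggered, sizes the target from area and resolution, gathers its own and linked actors' splines, and caches sampling center, size and yaw.
; Drawing renders triangles computed from selected splines, or composites stored textures instead, then optionally blurs the result.
; BeginPlay reinitializes and redraws after short random delays.
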(event EventBeginPlay
  (Utilities|FlowControl|Delay (Math|Random|RandomFloatinRange 0.0 0.5))
  (CallFunction|渲染资源初始化)
  (Utilities|FlowControl|Delay (Math|Random|RandomFloatinRange 0.0 0.5))
  (CallFunction|绘制 (Variables|区域控制|Get预览) (Variables|区域控制|Get使用贴图)))

(event Collision|EventActorBeginOverlap
  (params (OtherActor :type Actor%20Object%20Reference)))

(event EventTick
  (params (DeltaSeconds :type Float%20%28single-precision%29)))

(fn ConstructionScript
  (if (Variables|Default|Get实时刷新)
    (Utilities|FlowControl|Sequence :!label _label
      (:then_0
        (CallFunction|参数配置初始化)
        (CallFunction|渲染资源初始化))
      (:then_1
        (CallFunction|采集所有样条区域)
        (CallFunction|缓存采样参数))
      (:then_3
        (CallFunction|绘制 (Variables|区域控制|Get预览) (Variables|区域控制|Get使用贴图)))
      (:then_4
        (Variables|Default|Set手动刷新 false)))
    (elif (Variables|Default|Get手动刷新)
      (goto _label))))

(fn 参数配置初始化
  (bind _图像尺寸限制 (Variables|Default|Get图像尺寸限制))
  (bind _区域大小 (Variables|Default|Get区域大小))
  (bind _区域大小_2 (Variables|Default|Get区域大小))
  (bind _指定的贴图 (Variables|贴图设置|Get指定的贴图))
  (bind _分辨率 (Variables|贴图设置|Get分辨率))
  (bind _returnvalue (* _区域大小 1e+01))
  (bind _sizex (Variables|/Script/Engine.TextureRenderTarget2D|GetSizeX _指定的贴图))
  (bind _sizey (Variables|/Script/Engine.TextureRenderTarget2D|GetSizeY _指定的贴图))
  (bind _returnvalue_2 (Math|Integer|Max(Integer) _sizex _sizey))
  (bind _returnvalue_3 (* _returnvalue _分辨率))
  (bind _returnvalue_4 (Math|Float|Truncate _returnvalue_3))
  ;[1 1 1] h
  (Transformation|SetRelativeScale3D (Variables|Default|GetStaticMesh) (Math|Conversions|ToVector(Float) _区域大小_2))
  (Variables|计算缓存|Set世界采样大小 (* _区域大小_2 1e+02))
  (if (Variables|贴图设置|Get使用指定RT)
    (Variables|计算缓存|Set图像尺寸 _returnvalue_2)
    (Variables|计算缓存|Set样条点映射大小数值 (/ (* (Variables|Default|Get区域大小) 1e+02) _returnvalue_2))
    (elif (< _returnvalue_4 _图像尺寸限制)
      (Variables|计算缓存|Set图像尺寸 _returnvalue_4)
      (Variables|计算缓存|Set样条点映射大小数值 (* (/ 1.0 (Variables|贴图设置|Get分辨率)) 1e+01))
      (else
        (Variables|计算缓存|Set图像尺寸 (Math|Float|Truncate _图像尺寸限制))
        (Variables|计算缓存|Set样条点映射大小数值 (/ (* (Variables|Default|Get区域大小) 1e+02) (Variables|Default|Get图像尺寸限制)))))))

(fn 渲染资源初始化
  (bind _图像尺寸 (Variables|计算缓存|Get图像尺寸))
  (Utilities|FlowControl|Sequence
    (:then_0
      (if (Variables|贴图设置|Get使用指定RT)
        (bind _output_get (Variables|缓存|SetRenderTarget (Variables|贴图设置|Get指定的贴图)))
        (Rendering|ClearRenderTarget2D _output_get)
        (else
          (Utilities|IsValid (Variables|缓存|GetRenderTarget)
            (:Is%20Valid
              (Rendering|ClearRenderTarget2D (Variables|缓存|GetRenderTarget)))
            (:Is%20Not%20Valid
              (bind _returnvalue (Rendering|CreateRenderTarget2D _图像尺寸 _图像尺寸 "RTF_R8"))
              (Variables|缓存|SetRenderTarget _returnvalue))))))
    (:then_1
      (Utilities|IsValid (Variables|缓存|GetRTDebugMaterial)
        (:Is%20Not%20Valid
          (bind _returnvalue_2 (Rendering|Material|CreateDynamicMaterialInstance (Variables|Default|GetStaticMesh) 0 "/Game/LibSu/Asset/Material/M_RTDebug.M_RTDebug" "None" :!class /Script/Engine.PrimitiveComponent))
          (bind _output_get_2 (Variables|缓存|SetRTDebugMaterial _returnvalue_2))
          (Rendering|Material|SetTextureParameterValue _output_get_2 "RT" (Variables|缓存|GetRenderTarget)))))))

(fn 采集所有样条区域
  (bind _spline_set (Variables|计算缓存|GetSpline_Set))
  (Utilities|Array|Clear _spline_set)
  (Utilities|Array|Add _spline_set (Variables|Default|GetSpline))
  ;[1 1 1] 整理所有选中的actor的spline
  (for _array_element (Variables|区域控制|Get其他样条线)
    (Transformation|SetActorLocation _array_element (+ (Transformation|GetActorLocation) "0.000000,0.000000,1000.000000") false false)
    (Transformation|SetActorRotation _array_element (Transformation|GetActorRotation))
    (Utilities|Array|Add (Variables|计算缓存|GetSpline_Set) (Variables|/Game/LibSu/Asset/Actor/BP_Spline_Actor.BP_Spline_Actor_C|GetSpline _array_element))))

(fn 缓存采样参数
  (Variables|采样参数缓存|Set采样中心位置 (Transformation|GetActorLocation))
  (Variables|采样参数缓存|Set采样大小 (Variables|计算缓存|Get世界采样大小))
  (Variables|采样参数缓存|Set采样旋转 (/ (.yaw (Transformation|GetActorRotation)) -3.6e+02)))

(fn 绘制
  (params (绘制的索引 :type Array%20of%20Integers) (绘制贴图 :type Boolean))
  (Utilities|FlowControl|Sequence
    (:then_0
      (if 绘制贴图
        (Rendering|ClearRenderTarget2D (Variables|缓存|GetRenderTarget))
        (for _array_element 绘制的索引
          (CallFunction|贴图渲染到渲染目标 (Variables|缓存|GetRenderTarget) (Utilities|Array|Get(acopy) (Variables|区域控制|Get贴图) _array_element)))
        (else
          (bind _triangles1 (CallFunction|三角形计算渲染目标 绘制的索引 (Variables|计算缓存|GetSpline_Set) (Variables|区域控制|Get样条采样距离) (Variables|计算缓存|Get样条点映射大小数值) (Variables|计算缓存|Get图像尺寸)))
          (CallFunction|三角形渲染到渲染目标 (Variables|缓存|GetRenderTarget) _triangles1 "/Game/LibSu/Asset/Texture/T_White.T_White"))))
    (:then_1
      (if (not (<= (Variables|区域控制|Get模糊大小) 1.0))
        (CallFunction|模糊渲染目标贴图 (Variables|缓存|GetRenderTarget) (Variables|区域控制|Get模糊大小))))))