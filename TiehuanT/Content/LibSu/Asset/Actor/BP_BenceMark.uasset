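; BP_BenceMark is a benchmark actor that flies the player pawn along its spline while showing FPS stats.
; Event_BenchMark runs "stat fps" and plays a timeline at a rate set by the duration variable, or stops it when Run is false.
; Each update maps timeline alpha to spline distance and sets only the pawn's location, using the spline's local-space point as a world position.
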(event Custom|Event_BenchMark
  (params (Run :type Boolean))
  (bind _spline (Variables|Default|GetSpline))
  (if Run
    (Components|Timeline|SetPlayRate (Variables|Default|Get时间轴) (/ 1.0 (Variables|Default|Get播放时长)))
    (Development|ExecuteConsoleCommand "stat fps" 0)
    (bind _新建轨道_0 (Timeline|时间轴 Play)
      (:Update
        (Transformation|SetActorLocation (Game|Player|GetPlayerPawn 0) (Spline|GetLocationatDistanceAlongSpline _spline (Math|Float|Lerp 0.0 (Spline|GetSplineLength _spline) _新建轨道_0) "Local") false false)))
    (else
      (Utilities|FlowControl|Sequence
        (:then_0
          (Timeline|时间轴 Stop))))))

(event EventBeginPlay)

(event Collision|EventActorBeginOverlap
  (params (OtherActor :type Actor%20Object%20Reference)))

(event EventTick
  (params (DeltaSeconds :type Float%20%28single-precision%29)))

(fn ConstructionScript)